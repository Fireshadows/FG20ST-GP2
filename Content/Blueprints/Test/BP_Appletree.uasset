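; BP_Appletree is a test apple tree whose three child-actor apples cannot be dragged until a snappable object, apparently a ladder, is placed against it.
; On BeginPlay it disables the apples' BPAC_Draggable components and binds their uninteractable-drag event to a printed "cannot reach" message.
; When an actor with BPAC_Snappable enters TreeHitbox, it snaps to LadderSocket and the player's drag is cleared.
; If that actor is draggable, it gets locked and the apples become interactable.
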(event OnComponentBeginOverlap(TreeHitbox)
  (params (OverlappedComponent :type Primitive%20Component%20Object%20Reference) (OtherActor :type Actor%20Object%20Reference) (OtherComp :type Primitive%20Component%20Object%20Reference) (OtherBodyIndex :type Integer) (bFromSweep :type Boolean) (SweepResult :type Hit%20Result%20Structure%20%28by%20ref%29))
  (bind _returnvalue (Actor|GetComponentbyClass OtherActor "/Game/Blueprints/BPAC_Draggable.BPAC_Draggable_C"))
  (if (Utilities|IsValid (Actor|GetComponentbyClass OtherActor "/Game/Blueprints/BPAC_Snappable.BPAC_Snappable_C"))
    (Transformation|AttachActorToActor OtherActor self "LadderSocket" "SnapToTarget" "SnapToTarget" "SnapToTarget" true)
    (bind _asbp_character (Utilities|Casting|CastToBP_Character (Game|Player|GetPlayerPawn 0)))
    (Variables|/Game/Blueprints/Core/BP_Character.BP_Character_C|SetMouseClicked _asbp_character false)
    (Variables|/Game/Blueprints/Core/BP_Character.BP_Character_C|SetDraggingComponent _asbp_character 0)
    (if (Utilities|IsValid _returnvalue)
      (Variables|/Script/FGGP2.InteractBaseComponent|Setinteractable _returnvalue false)
      (CallFunction|SetChildInteractability true))))

(event Custom|OnGrabbingUnavailableApple
  (Development|PrintString "Cannot reach these apples!"))

(event EventBeginPlay
  (Variables|Default|SetApples (Utilities|Array|MakeArray (Variables|/Script/Engine.ChildActorComponent|GetChildActor (Variables|Default|GetApple)) (Variables|/Script/Engine.ChildActorComponent|GetChildActor (Variables|Default|GetApple1)) (Variables|/Script/Engine.ChildActorComponent|GetChildActor (Variables|Default|GetApple2))))
  (CallFunction|SetChildInteractability false)
  (for _array_element (Variables|Default|GetApples)
    (if (Utilities|IsValid (Actor|GetComponentbyClass _array_element "/Game/Blueprints/BPAC_Draggable.BPAC_Draggable_C"))
      (EventDispatchers|BindEventtoOnDragUninteractable (Actor|GetComponentbyClass _array_element "/Game/Blueprints/BPAC_Draggable.BPAC_Draggable_C") (delegate Custom|OnGrabbingUnavailableApple)))))

(fn ConstructionScript)

(fn SetChildInteractability
  (params (Become%20Interactable :type Boolean))
  (for _array_element (Variables|Default|GetApples)
    (bind _asbp_apple (Utilities|Casting|CastToBP_Apple _array_element))
    (Variables|/Script/FGGP2.InteractBaseComponent|Setinteractable (Actor|GetComponentbyClass _asbp_apple "/Game/Blueprints/BPAC_Draggable.BPAC_Draggable_C") Become%20Interactable)))