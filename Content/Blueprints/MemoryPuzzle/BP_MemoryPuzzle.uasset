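; BP_MemoryPuzzle is a piece in a memory puzzle that hides a text label behind a sliding curtain.
; On BeginPlay it copies its Memory value into the BPACMemory component's TextState and displays that enum as text.
; RevealObject and HideObject run timelines that nudge the curtain in opposite directions each update, blocking clicks until finished.
; StayRevealed marks the component completed and disables clicking.
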(event Custom|HideObject
  (Variables|Default|SetAcceptClicking false)
  (Timeline|Timeline_1 PlayFromStart
    (:Update
      (Transformation|AddLocalOffset (Variables|Default|GetCurtain) "2.500000,0.000000,0.000000" false false))
    (:Finished
      (Variables|Default|SetAcceptClicking true))))

(event Custom|StayRevealed
  (Variables|/Game/Blueprints/BPAC_MemoryObject.BPAC_MemoryObject_C|SetCompleted (Variables|Default|GetBPAC_Memory) true)
  (Variables|Default|SetAcceptClicking false))

(event Custom|RevealObject
  (params (ComparedObject :type BPAC%20Memory%20Object%20Object%20Reference))
  (Variables|Default|SetAcceptClicking false)
  (Timeline|Timeline_0 PlayFromStart
    (:Update
      (Transformation|AddLocalOffset (Variables|Default|GetCurtain) "-2.500000,0.000000,0.000000" false false))
    (:Finished
      (Variables|Default|SetAcceptClicking true))))

(event EventBeginPlay
  (bind _output_get (Variables|/Game/Blueprints/BPAC_MemoryObject.BPAC_MemoryObject_C|SetTextState (Variables|Default|GetBPAC_Memory) (Variables|Default|GetMemory)))
  (Rendering|Components|TextRender|SetText (Variables|Default|GetTextRender) (Utilities|Text|ToText(String) (Utilities|String|EnumtoString _output_get))))

(fn ConstructionScript)