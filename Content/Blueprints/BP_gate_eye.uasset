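; BP_gate_eye is a gate eye that animates its gaze by writing random X and Y scalar parameters to its static mesh's materials.
; On Tick, the Stabbed flag, not set in this Blueprint, selects rapid jitter that flips between positive and negative offsets every frame.
; Otherwise, Delay nodes pace smaller alternating glances, which later reset X and Y to center and set the UV parameter.
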(event EventTick
  (params (DeltaSeconds :type Float%20%28single-precision%29))
  (bind _returnvalue (Math|Random|RandomFloatinRange 0.0 -0.001))
  (bind _returnvalue_2 (Math|Random|RandomFloatinRange 0.001 0.01))
  (bind _returnvalue_3 (Math|Random|RandomFloatinRange 0.0 0.001))
  (bind _staticmesh (Variables|Default|GetStaticMesh))
  (bind _returnvalue_4 (* _returnvalue_2 -1.0))
  (if (Variables|Default|GetStabbed?)
    ;[1 1 1] Stabbed Eye Movement
    (Utilities|FlowControl|FlipFlop
      (:A
        (Rendering|Material|SetScalarParameterValueonMaterials _staticmesh "Y" _returnvalue_2)
        (Rendering|Material|SetScalarParameterValueonMaterials _staticmesh "X" _returnvalue_2))
      (:B
        (Rendering|Material|SetScalarParameterValueonMaterials _staticmesh "Y" _returnvalue_4)
        (Rendering|Material|SetScalarParameterValueonMaterials _staticmesh "X" _returnvalue_4)))
    (else
      (Utilities|FlowControl|Delay (Math|Random|RandomFloatinRange 1.0 2.0))
      (Utilities|FlowControl|FlipFlop
        (:A
          (Rendering|Material|SetScalarParameterValueonMaterials _staticmesh "Y" _returnvalue_3)
          (Rendering|Material|SetScalarParameterValueonMaterials _staticmesh "X" _returnvalue_3)
          (Utilities|FlowControl|Delay 1e+01))
        (:B
          (Rendering|Material|SetScalarParameterValueonMaterials _staticmesh "Y" _returnvalue)
          (Rendering|Material|SetScalarParameterValueonMaterials _staticmesh "X" _returnvalue)
          (Utilities|FlowControl|Delay 1e+01)))
      (Rendering|Material|SetScalarParameterValueonMaterials _staticmesh "Y" 0.0)
      (Rendering|Material|SetScalarParameterValueonMaterials _staticmesh "X" 0.0)
      (Rendering|Material|SetScalarParameterValueonMaterials _staticmesh "UV" 1.0))))

(fn ConstructionScript)