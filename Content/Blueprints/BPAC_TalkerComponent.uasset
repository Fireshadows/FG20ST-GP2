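; Actor component that displays a talking actor's subtitle lines in an on-screen text box and plays each line's optional sound.
; On subtitle start it borrows a box from WBP_TalkerManager, releasing it on finish.
; Each line is placed at the owner's projected screen position, relative to viewport center, when shown.
; Subtitle events drive the display, fixed-duration lines start a timer, and clicks are forwarded until talking finishes.
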(event EventBeginPlay
  (Utilities|FlowControl|Delay 0.2)
  (CallFunction|SetTalkerManagerReference)
  (|SubtitleEventBinding))

(event EventTick
  (params (DeltaSeconds :type Float%20%28single-precision%29)))

(event EventClickable
  (if (not (Variables|Default|GetFinishedTalking?))
    (Class|SubtitleComponent|Clicked)))

(fn ManageSubtitleEventImpl
  (params (SubtitleEvent :type ESubtitleEvent%20Enum :default "SubtitleFinished"))
  (switch Utilities|FlowControl|Switch|SwitchonESubtitleEvent SubtitleEvent
    (:SubtitleFinished
      (CallFunction|StopShowingText)
      (Default|CallFinishedTalking)
      (Variables|Default|SetFinishedTalking? true))
    (:SubtitleStarted
      (CallFunction|StartShowingText))
    (:SubtitleNext
      (CallFunction|NewTexttoShow))))

(fn SetTalkerManagerReference
  (bind _foundwidgets (Widget|GetAllWidgetsOfClass "/Game/Blueprints/UI/Text/WBP_TalkerManager.WBP_TalkerManager_C" false))
  (Variables|Default|SetTalkerManager (Utilities|Array|Get(acopy) _foundwidgets)))

(fn StartShowingText
  (if (Utilities|IsValid (Variables|Default|GetCurrentlyUsedTextBox))
    _
    (else
      (bind _freewidget (Default|GetTextBox (Variables|Default|GetTalkerManager)))
      (Variables|Default|SetCurrentlyUsedTextBox _freewidget)))
  (Class|BPITextBoxInterface|ShowWidget(Message) (Variables|Default|GetCurrentlyUsedTextBox))
  (CallFunction|ShowTextImpl)
  (CallFunction|HandleNextText))

(fn StopShowingText
  (if (Utilities|IsValid (Variables|Default|GetCurrentlyUsedTextBox))
    (Default|ReleaseTextBox (Variables|Default|GetTalkerManager) (Variables|Default|GetCurrentlyUsedTextBox))))

(fn HandleNextText
  (bind _returnvalue (Class|SubtitleComponent|GetCurrentTextData))
  (switch Utilities|FlowControl|Switch|SwitchonENextLineTrigger (.triggerType (Utilities|Struct|BreakTextData _returnvalue))
    (:OnFixedDuration
      _)
    (:OnFixedDurationOrClick
      _))
  (Class|SubtitleComponent|StartTimer (.duration (Utilities|Struct|BreakTextData _returnvalue))))

(fn GetActorLocationinViewport
  (params (Actor :type Actor%20Object%20Reference))
  (bind _returnvalue (Game|GetPlayerController 0))
  (bind _returnvalue_2 (Transformation|GetActorLocation Actor))
  (bind (_screenlocation _returnvalue_3) (Class|PlayerController|ProjectWorldLocationtoScreen _returnvalue _returnvalue_2 false))
  (bind (_sizex _sizey) (HUD|GetViewportSize _returnvalue))
  (return (- _screenlocation (* (Math|Vector2D|MakeVector2D (Math|Conversions|ToFloat(Integer) _sizex) (Math|Conversions|ToFloat(Integer) _sizey)) 0.5)) _returnvalue_3))

(fn ShowTextImpl
  (bind _returnvalue (Class|SubtitleComponent|GetCurrentTextData))
  (Class|BPITextBoxInterface|SetText(Message) (Variables|Default|GetCurrentlyUsedTextBox) (.line (Utilities|Struct|BreakTextData _returnvalue)))
  (if (Utilities|IsValid (.soundRef (Utilities|Struct|BreakTextData _returnvalue)))
    (Audio|PlaySound2D (.soundRef (Utilities|Struct|BreakTextData _returnvalue)) 1.0 1.0 0.0 0 0))
  (bind _viewport_position (CallFunction|GetActorLocationinViewport (Components|GetOwner)))
  (Class|BPITextBoxInterface|SetPosition(Message) (Variables|Default|GetCurrentlyUsedTextBox) _viewport_position)
  (return))

(fn NewTexttoShow
  (CallFunction|ShowTextImpl)
  (CallFunction|HandleNextText))

(event Custom|ManageSubtitles
  (params (SubtitleEvent :type ESubtitleEvent%20Enum :default "SubtitleFinished"))
  (CallFunction|ManageSubtitleEventImpl SubtitleEvent))