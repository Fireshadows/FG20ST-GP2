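; A single tile of the Room 2 memory puzzle, with blinds that slide to reveal or hide its object.
; BeginPlay labels it from the BPACMemory component, whose Completed flag StayRevealed sets while disabling clicks.
; Reveal and hide lerp the blinds through timelines with a panel sound, blocking clicks until finished; two generically named events repeat this silently.
; Hover events toggle custom depth on the blinds for highlighting.
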(event Custom|HideObject
  (Variables|Default|SetAcceptClicking false)
  (Variables|Default|SetTargetCurtainLocation (Variables|Default|GetOldCurtainLocation))
  (Variables|Default|SetOldCurtainLocation (Transformation|GetWorldLocation (Variables|Default|GetBlinds)))
  (Audio|PlaySound2D "/Game/Assets/Sound/Trigger/Flavor/sound_TemplePanels.sound_TemplePanels" 1.0 1.0 0.0 0 0)
  (bind _alpha (Timeline|Timeline_2 PlayFromStart)
    (:Update
      (Transformation|SetWorldLocation (Variables|Default|GetBlinds) (Math|Vector|Lerp(Vector) (Variables|Default|GetOldCurtainLocation) (Variables|Default|GetTargetCurtainLocation) _alpha) false false))
    (:Finished
      (Variables|Default|SetAcceptClicking true))))

(event Custom|StayRevealed
  (Variables|/Game/Blueprints/ActorComponents/BPAC_MemoryObject.BPAC_MemoryObject_C|SetCompleted (Variables|Default|GetBPAC_Memory) true)
  (Variables|Default|SetAcceptClicking false))

(event Custom|RevealObject
  (params (ComparedObject :type BPAC%20Memory%20Object%20Object%20Reference))
  (Variables|Default|SetAcceptClicking false)
  (Variables|Default|SetOldCurtainLocation (Transformation|GetWorldLocation (Variables|Default|GetBlinds)))
  (Audio|PlaySound2D "/Game/Assets/Sound/Trigger/Flavor/sound_TemplePanels.sound_TemplePanels" 1.0 1.0 0.0 0 0)
  (bind _alpha (Timeline|Timeline_0 PlayFromStart)
    (:Update
      (Transformation|SetWorldLocation (Variables|Default|GetBlinds) (Math|Vector|Lerp(Vector) (Variables|Default|GetOldCurtainLocation) (Math|Vector|MakeVector (.X (Math|Vector|BreakVector (Variables|Default|GetOldCurtainLocation))) (.Y (Math|Vector|BreakVector (Variables|Default|GetOldCurtainLocation))) (+ (.Z (Math|Vector|BreakVector (Variables|Default|GetOldCurtainLocation))) (Variables|Default|GetCurtainOffset))) _alpha) false false))
    (:Finished
      (Variables|Default|SetAcceptClicking true))))

(event Custom|CustomEvent
  (params (ComparedObject :type BPAC%20Memory%20Object%20Object%20Reference))
  (Variables|Default|SetAcceptClicking false)
  (Variables|Default|SetTargetCurtainLocation (Variables|Default|GetOldCurtainLocation))
  (Variables|Default|SetOldCurtainLocation (Transformation|GetWorldLocation (Variables|Default|GetBlinds)))
  (bind _alpha (Timeline|Timeline_3 PlayFromStart)
    (:Update
      (Transformation|SetWorldLocation (Variables|Default|GetBlinds) (Math|Vector|Lerp(Vector) (Variables|Default|GetOldCurtainLocation) (Variables|Default|GetTargetCurtainLocation) _alpha) false false))
    (:Finished
      (Variables|Default|SetAcceptClicking true))))

(event Custom|CustomEvent_1
  (Variables|Default|SetAcceptClicking false)
  (Variables|Default|SetOldCurtainLocation (Transformation|GetWorldLocation (Variables|Default|GetBlinds)))
  (bind _alpha (Timeline|Timeline_1 PlayFromStart)
    (:Update
      (Transformation|SetWorldLocation (Variables|Default|GetBlinds) (Math|Vector|Lerp(Vector) (Variables|Default|GetOldCurtainLocation) (Math|Vector|MakeVector (.X (Math|Vector|BreakVector (Variables|Default|GetOldCurtainLocation))) (.Y (Math|Vector|BreakVector (Variables|Default|GetOldCurtainLocation))) (+ (.Z (Math|Vector|BreakVector (Variables|Default|GetOldCurtainLocation))) 1.0)) _alpha) false false))
    (:Finished
      (Variables|Default|SetAcceptClicking true))))

(event EventStartHovering
  (Rendering|SetRenderCustomDepth (Variables|Default|GetBlinds) true))

(event EventStopHovering
  (Rendering|SetRenderCustomDepth (Variables|Default|GetBlinds) false))

(event EventBeginPlay
  (bind _output_get (Variables|/Game/Blueprints/ActorComponents/BPAC_MemoryObject.BPAC_MemoryObject_C|SetTextState (Variables|Default|GetBPAC_Memory) (Variables|Default|GetMemory)))
  (Rendering|Components|TextRender|SetText (Variables|Default|GetTextRender) (Utilities|Text|ToText(String) _output_get))
  (Components|Timeline|SetPlayRate (Variables|Default|GetTimeline_2) (Variables|Default|GetCurtainMovementSpeed))
  (Variables|Default|SetAcceptClicking true))

(fn ConstructionScript)