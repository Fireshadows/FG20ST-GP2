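; Anubis actor for a judgement scene that weighs the player's fate, spawning a heart and a feather at offsets from itself on BeginPlay.
; Judgement reads FatePoints from BP_Gamestate, then plays a timeline that shifts both props along local negative Z by a fixed step each update.
; When it finishes, the narrator advances zero, one or two times according to the neutral and good thresholds, then starts.
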(event Custom|Judgement
  (bind _bpac_narrator (Variables|Default|GetBPAC_Narrator))
  (bind _asbp_gamestate (Utilities|Casting|CastToBP_Gamestate (Game|GetGameState)))
  (Variables|Default|SetFatePoints (Variables|/Game/Blueprints/Core/BP_Gamestate.BP_Gamestate_C|GetFatePoints _asbp_gamestate))
  (Timeline|Timeline_0 PlayFromStart
    (:Update
      (Transformation|AddActorLocalOffset (Variables|Default|GetHeart) "0, 0,-2.000000" false false)
      (Transformation|AddActorLocalOffset (Variables|Default|GetFeather) "0, 0,-2.000000" false false))
    (:Finished
      (if (< (Variables|Default|GetFatePoints) (Variables|Default|GetNeutralThreshold))
        _
        (else
          (Class|SubtitleComponent|Next _bpac_narrator)
          (if (>= (Variables|Default|GetFatePoints) (Variables|Default|GetGoodThreshold))
            (Class|SubtitleComponent|Next _bpac_narrator))))
      (Class|SubtitleComponent|Start _bpac_narrator))))

(event EventBeginPlay
  (bind _returnvalue (Transformation|GetActorTransform))
  (bind _returnvalue_2 (Transformation|GetActorTransform))
  (bind _location (Math|Transform|BreakTransform _returnvalue))
  (bind _location_2 (Math|Transform|BreakTransform _returnvalue_2))
  (bind (_x _y _z) (Math|Vector|BreakVector _location_2))
  (bind (_x_2 _y_2 _z_2) (Math|Vector|BreakVector _location))
  (bind _returnvalue_3 (Game|SpawnActorfromClass "/Game/Blueprints/Room4Anubis/BP_Heart.BP_Heart_C" (Math|Transform|MakeTransform (Math|Vector|MakeVector _x_2 (+ _y_2 1e+02) (+ _z_2 2e+02)) "0.000000,180.000000,0.000000") "Undefined" 0 0))
  (Variables|Default|SetHeart _returnvalue_3)
  (bind _returnvalue_4 (Game|SpawnActorfromClass "/Game/Blueprints/Room4Anubis/BP_Feather.BP_Feather_C" (Math|Transform|MakeTransform (Math|Vector|MakeVector _x (+ _y 3e+02) (+ _z 2e+02)) "0,180.000000, 0" "1,1.000000,1") "Undefined" 0 0))
  (Variables|Default|SetFeather _returnvalue_4))

(fn ConstructionScript)