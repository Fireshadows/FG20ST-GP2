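; Cerberus character that poses a one-time item choice in its room, resolved by overlapping it with a corpse or flute.
; At the dialogue branch, the accepted item is destroyed and enters its keyword to pick the fed or sleep line; only the flute counts as the good choice.
; When dialogue stops, it reports room completion and the fate choice to BP_Gamestate, where it registers itself on BeginPlay.
; Clicks play the talking animation for the sound component's timer.
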(event AnimatedTextLineFinished(BPAC_DialogueComponent))

(event AnimatedTextLineStarted(BPAC_DialogueComponent))

(event DialogueStarted(BPAC_DialogueComponent))

(event DialogueNext(BPAC_DialogueComponent))

(event DialogueStopped(BPAC_DialogueComponent)
  (bind _gamestate (Variables|Default|GetGameState))
  (Default|OnRoomFinished _gamestate)
  (Default|UpdateFatePoint _gamestate (Variables|Default|GetbGoodChoice)))

(event Custom|Clicked
  (Default|PlayAnimation (Variables|Default|GetBPAC_TalkingAnim))
  (Utilities|FlowControl|Delay (Variables|/Game/Blueprints/ActorComponents/BPAC_Sound.BPAC_Sound_C|GetTimer (Variables|Default|GetBPAC_Sound)))
  (Default|StopAnimation (Variables|Default|GetBPAC_TalkingAnim)))

(event Custom|CerberusFed
  (Class|DialogueComponent|EnterKeyword (Variables|Default|GetBPAC_DialogueComponent) (Variables|Default|GetCorpseKeyword)))

(event Custom|CerberusSleeped
  (Class|DialogueComponent|EnterKeyword (Variables|Default|GetBPAC_DialogueComponent) (Variables|Default|GetFluteKeyword))
  (Variables|Default|SetbGoodChoice true))

(event EventBeginPlay
  (EventDispatchers|BindEventtoClicked (Variables|Default|GetBPAC_Sound) (delegate Custom|Clicked))
  (bind _asbp_gamestate (Utilities|Casting|CastToBP_Gamestate (Game|GetGameState)))
  (bind _output_get (Variables|Default|SetGameState _asbp_gamestate))
  (Variables|/Game/Blueprints/Core/BP_Gamestate.BP_Gamestate_C|SetCerberus _output_get self)
  (CallFunction|SetupText))

(event Collision|EventActorBeginOverlap
  (params (OtherActor :type Actor%20Object%20Reference))
  (bind _returnvalue (Utilities|GetClass OtherActor))
  (if (Class|DialogueComponent|AtBranch (Variables|Default|GetBPAC_DialogueComponent))
    (if (not (Variables|Default|GetbSatisfied))
      (if (== _returnvalue "/Game/Blueprints/Room3/BP_Corpse.BP_Corpse_C")
        (CallFunction|CerberusFed)
        (Actor|DestroyActor OtherActor :!label _label)
        (Variables|Default|SetbSatisfied true)
        (elif (== _returnvalue "/Game/Blueprints/Room2/BP_Flute.BP_Flute_C")
          (CallFunction|CerberusSleeped)
          (goto _label))))))

(fn ConstructionScript)

(fn StartTalking
  (Class|DialogueComponent|Start (Variables|Default|GetBPAC_DialogueComponent)))

(fn SetupText
  (bind _returnvalue (Class|DialogueComponent|InitializeText (Variables|Default|GetBPAC_DialogueComponent) "Grr, woof, woof." 0.0))
  (bind _returnvalue_2 (Class|DialogueComponent|AddBranch (Variables|Default|GetBPAC_DialogueComponent) _returnvalue))
  (Utilities|FlowControl|Sequence
    (:then_0
      (Class|DialogueComponent|AddLinetoBranch (Variables|Default|GetBPAC_DialogueComponent) _returnvalue_2 (Utilities|Struct|MakeBranchInput (Variables|Default|GetCorpseKeyword) "Munch, crunch.") 3.0))
    (:then_1
      (Class|DialogueComponent|AddLinetoBranch (Variables|Default|GetBPAC_DialogueComponent) _returnvalue_2 (Utilities|Struct|MakeBranchInput (Variables|Default|GetFluteKeyword) "Zzz…") 3.0))))