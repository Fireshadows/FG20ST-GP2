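; BP_Vessel is a clickable character that carries a hint and plays a talking animation when clicked.
; On BeginPlay it passes the hint to its dialogue component and binds its click handler to the sound component.
; A click runs the talking animation component for the length of the sound component's timer.
; Hover events toggle custom depth rendering on the skeletal mesh as a highlight hook.
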(event Custom|Clicked
  (Default|PlayAnimation (Variables|Default|GetBPAC_TalkingAnim))
  (Utilities|FlowControl|Delay (Variables|/Game/Blueprints/ActorComponents/BPAC_Sound.BPAC_Sound_C|GetTimer (Variables|Default|GetBPAC_Sound)))
  (Default|StopAnimation (Variables|Default|GetBPAC_TalkingAnim)))

(event EventBeginPlay
  (EventDispatchers|BindEventtoClicked (Variables|Default|GetBPAC_Sound) (delegate Custom|Clicked))
  (Class|DialogueComponent|InitializeText (Variables|Default|GetBPAC_DialogueComponent) (Variables|Default|GetHintToGive) 5.0))

(event EventStopHovering
  (Rendering|SetRenderCustomDepth (Variables|Default|GetSkeletalMesh) false))

(event EventStartHovering
  (Rendering|SetRenderCustomDepth (Variables|Default|GetSkeletalMesh) true))

(fn ConstructionScript)