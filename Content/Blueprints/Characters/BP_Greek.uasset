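; Greek character that moves through scripted target points past a window, out of view, to a door and outside as completed matches increase.
; MovePosition picks a stage from the match count, using timelines to lerp location while advancing talker dialogue, and spawns BP_Flute after the last move.
; Overlapping a BP_SinObject compares sins and swaps the dialogue asset; a correct match also destroys both actors and updates the game state's fate point.
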(event Custom|MovePosition
  (params (CompletedMatches :type Integer))
  (switch int CompletedMatches
    (:1
      (Variables|Default|SetCurrentTarget (Transformation|GetActorLocation (Variables|Default|GetTargetPoint1PastWindow)))
      (Utilities|FlowControl|Sequence ; Seq because text appears during movement
        (:then_0
          (Timeline|MovementPastWindow PlayFromStart
            (:Update
              (Transformation|SetActorLocation (Math|Vector|Lerp(Vector) (Transformation|GetActorLocation) (Variables|Default|GetCurrentTarget) 0.1) false false))
            (:Finished
              (Variables|Default|SetCurrentTarget (Transformation|GetActorLocation (Variables|Default|GetTargetPoint2Window))))))
        (:then_1
          (Utilities|FlowControl|Delay 0.4)
          (Class|SubtitleComponent|Start (Variables|Default|GetBPAC_TalkerComponent))
          (Variables|Default|SetStarted true))))
    (:2
      (Timeline|MovementToWindow PlayFromStart
        (:Update
          (Transformation|SetActorLocation (Math|Vector|Lerp(Vector) (Transformation|GetActorLocation) (Variables|Default|GetCurrentTarget) 0.1) false false))
        (:Finished
          (Class|SubtitleComponent|Next (Variables|Default|GetBPAC_TalkerComponent))
          (Variables|Default|SetCurrentTarget (Transformation|GetActorLocation (Variables|Default|GetTargetPoint3OutofView))))))
    (:3
      (Class|SubtitleComponent|Next (Variables|Default|GetBPAC_TalkerComponent))
      (Timeline|MovementOutOfView PlayFromStart
        (:Update
          (Transformation|SetActorLocation (Math|Vector|Lerp(Vector) (Transformation|GetActorLocation) (Variables|Default|GetCurrentTarget) 0.1) false false))
        (:Finished
          (Variables|Default|SetCurrentTarget (Transformation|GetActorLocation (Variables|Default|GetTargetPoint4Door)))
          (Transformation|SetActorLocation (Transformation|GetActorLocation (Variables|Default|GetTargetPoint3,5)) false false))))
    (:4
      (Timeline|Timeline_0 PlayFromStart
        (:Update
          (Transformation|SetActorLocation (Math|Vector|Lerp(Vector) (Transformation|GetActorLocation) (Variables|Default|GetCurrentTarget) 0.1) false false))
        (:Finished
          (Class|SubtitleComponent|Next (Variables|Default|GetBPAC_TalkerComponent))
          (Variables|Default|SetCurrentTarget (Transformation|GetActorLocation (Variables|Default|GetTargetPoint5Outside)))
          (Timeline|Timeline_1 PlayFromStart
            (:Update
              (Transformation|SetActorLocation (Math|Vector|Lerp(Vector) (Transformation|GetActorLocation) (Variables|Default|GetCurrentTarget) 0.1) false false))
            (:Finished
              (Game|SpawnActorfromClass "/Game/Blueprints/Room2/BP_Flute.BP_Flute_C" (Math|Transform|MakeTransform "1230.000000,-520.000000,1690.000000" "0.000000,80.000000, 0" "0.200000,0.200000,0.200000") "Undefined" 0 0))))))))

(event EventBeginPlay
  (Variables|Default|SetOriginalPosition (Transformation|GetActorLocation)))

(event Collision|EventActorBeginOverlap
  (params (OtherActor :type Actor%20Object%20Reference))
  (bind _bpac_talkercomponent (Variables|Default|GetBPAC_TalkerComponent))
  (bind _bpac_talkercomponent_2 (Variables|Default|GetBPAC_TalkerComponent))
  (if (== (Utilities|GetClass OtherActor) "/Game/Blueprints/BP_SinObject.BP_SinObject_C")
    (bind _asbp_sin_object (Utilities|Casting|CastToBP_SinObject OtherActor))
    (if (Utilities|Enum|Equal(Enum) (Variables|Default|GetAssociatedSin) (Variables|/Game/Blueprints/BP_SinObject.BP_SinObject_C|GetAssociatedSin _asbp_sin_object))
      (Variables|/Script/FGGP2.SubtitleComponent|SetDataAsset _bpac_talkercomponent "/Game/Data/Subtitles/SinCharacters/DA_SinGreekRightSin.DA_SinGreekRightSin")
      (Class|SubtitleComponent|Ended _bpac_talkercomponent_2)
      (Actor|DestroyActor OtherActor)
      (Actor|DestroyActor)
      (bind _asbp_gamestate (Utilities|Casting|CastToBP_Gamestate (Game|GetGameState)))
      (Default|UpdateFatePoint _asbp_gamestate true)
      (else
        (Variables|/Script/FGGP2.SubtitleComponent|SetDataAsset _bpac_talkercomponent "/Game/Data/Subtitles/SinCharacters/DA_SinGreekWrongSin.DA_SinGreekWrongSin")))
    (Class|SubtitleComponent|Start _bpac_talkercomponent_2)))

(fn ConstructionScript)