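; BP_Monk is an NPC who hints at a hunt to match sin-labelled scrolls with their owners.
; Dialogue, sound and talking-animation components drive its speech, with a restartable timer hiding the dialogue, which also hides at branches.
; Receiving a BP_SinObject with its associated sin enters the keyword for the branch line, destroys the item and updates the GameState's fate point.
; Hovering toggles custom depth on the mesh.
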(event DialogueNext(BPAC_DialogueComponent)
  (bind _bpac_dialoguecomponent (Variables|Default|GetBPAC_DialogueComponent))
  (Utilities|Time|ClearandInvalidateTimerbyHandle (Variables|Default|GetTimerHandle))
  (bind _returnvalue (Utilities|Time|SetTimerbyEvent (delegate Custom|HideTemp) (Variables|Default|GetTimeUntilHide)))
  (Variables|Default|SetTimerHandle _returnvalue)
  (if (Class|DialogueComponent|AtBranch _bpac_dialoguecomponent)
    (Default|HideTemporary _bpac_dialoguecomponent)))

(event DialogueReset(BPAC_DialogueComponent)
  (Default|HideTemporary (Variables|Default|GetBPAC_DialogueComponent)))

(event DialogueStarted(BPAC_DialogueComponent)
  (bind _bpac_dialoguecomponent (Variables|Default|GetBPAC_DialogueComponent))
  (bind _returnvalue (Utilities|Time|SetTimerbyEvent (delegate Custom|HideTemp) (Variables|Default|GetTimeUntilHide)))
  (Variables|Default|SetTimerHandle _returnvalue)
  (if (Class|DialogueComponent|AtBranch _bpac_dialoguecomponent)
    (Default|HideTemporary _bpac_dialoguecomponent)))

(event Custom|Clicked
  (Default|PlayAnimation (Variables|Default|GetBPAC_TalkingAnim))
  (Utilities|FlowControl|Delay (Variables|/Game/Blueprints/ActorComponents/BPAC_Sound.BPAC_Sound_C|GetTimer (Variables|Default|GetBPAC_Sound)))
  (Default|StopAnimation (Variables|Default|GetBPAC_TalkingAnim)))

(event Custom|HideTemp
  (Default|HideTemporary (Variables|Default|GetBPAC_DialogueComponent)))

(event EventBeginPlay
  (EventDispatchers|BindEventtoClicked (Variables|Default|GetBPAC_Sound) (delegate Custom|Clicked))
  (CallFunction|SetupText)
  (bind _asbp_gamestate (Utilities|Casting|CastToBP_Gamestate (Game|GetGameState)))
  (Variables|Default|SetGameState _asbp_gamestate))

(event EventStopHovering
  (Rendering|SetRenderCustomDepth (Variables|Default|GetStaticMesh) false))

(event EventStartHovering
  (Rendering|SetRenderCustomDepth (Variables|Default|GetStaticMesh) true))

(fn ConstructionScript)

(fn SetupText
  (bind _bpac_dialoguecomponent (Variables|Default|GetBPAC_DialogueComponent))
  (bind _returnvalue (Class|DialogueComponent|InitializeText _bpac_dialoguecomponent "This place isn't so bad, really. Less rules down here for starters!" 0.0))
  (bind _returnvalue_2 (Class|DialogueComponent|AddLine _bpac_dialoguecomponent _returnvalue "I've been seeing these scroll things around labled after people's sins. I think it's a treasure hunt or something to match them with their owner." 1e+01))
  (Class|DialogueComponent|AddReturnNode _bpac_dialoguecomponent _returnvalue_2)
  (Class|DialogueComponent|AddLinetoBranch _bpac_dialoguecomponent _returnvalue_2 (Utilities|Struct|MakeBranchInput (Variables|Default|GetRightKey) "You got me! Hehehe.") 2.0))

(fn ReceiveItem
  (params (Actor :type Actor%20Object%20Reference) (Collider :type Actor%20Component%20Object%20Reference))
  (bind _asbp_sin_object (Utilities|Casting|CastToBP_SinObject Actor)
    (:then
      (if (Utilities|Enum|Equal(Enum) (Variables|Default|GetAssociatedSin) (Variables|/Game/Blueprints/BP_SinObject.BP_SinObject_C|GetAssociatedSin _asbp_sin_object))
        (Class|DialogueComponent|EnterKeyword (Variables|Default|GetBPAC_DialogueComponent) (Variables|Default|GetRightKey))
        (Actor|DestroyActor Actor)
        (Default|UpdateFatePoint (Variables|Default|GetGameState) true)
        (return true)))
    (:CastFailed
      (return false))))