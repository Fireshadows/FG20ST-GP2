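; BPAC_TalkingAnim is an actor component that fakes a talking animation by pulsing the owning actor's scale.
; On BeginPlay it starts a looping timer at the Time interval, with an initial start delay of half that interval.
; Each tick of the timer flip-flops the owner's scale between OriginalScale plus ScaleOffset and OriginalScale, snapping without interpolation.
; OriginalScale is hardcoded to unit scale rather than read from the owner.
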(event Custom|ScaleAnim
  (bind _original_scale (Variables|Default|GetOriginal%20Scale))
  (Utilities|FlowControl|FlipFlop
    (:A
      (Variables|Default|SetTarget%20Scale (+ _original_scale (Variables|Default|GetScaleOffset))))
    (:B
      (Variables|Default|SetTarget%20Scale _original_scale)))
  (Transformation|SetActorScale3D (Components|GetOwner) (Variables|Default|GetTarget%20Scale)))

(event EventBeginPlay
  (bind _time (Variables|Default|GetTime))
  (Variables|Default|SetOriginal%20Scale "1.000000,1.000000,1.000000")
  (Utilities|Time|SetTimerbyEvent (delegate Custom|ScaleAnim) _time true (* _time 0.5)))