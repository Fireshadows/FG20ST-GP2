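; Dialogue actor component that displays timed, branching lines in either the narrator subtitle box or a talker text box obtained from the talker manager widget.
; Dialogue start, next and stop events drive widget setup, text updates, per-line timers and cleanup, though StartTalking always calls show on the narrator widget.
; BeginPlay currently builds a placeholder branching test dialogue and starts it after a short delay.
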(event Custom|NextEvent
  (Utilities|Time|ClearandInvalidateTimerbyHandle (Variables|Default|GetNextLineTimer))
  (CallFunction|NextLine))

(event Custom|StartedEvent
  (CallFunction|StartTalking))

(event Custom|StoppedEvent
  (CallFunction|StopTalking)
  (Utilities|Time|ClearandInvalidateTimerbyHandle (Variables|Default|GetNextLineTimer)))

(event EventBeginPlay
  (EventDispatchers|BindEventtoDialogueNext (delegate Custom|NextEvent))
  (EventDispatchers|BindEventtoDialogueStarted (delegate Custom|StartedEvent))
  (EventDispatchers|BindEventtoDialogueStopped (delegate Custom|StoppedEvent))
  (CallFunction|TestText)
  (Utilities|FlowControl|Delay 3.0)
  (Class|DialogueComponent|Start))

(fn StartTalking
  (CallFunction|InitializeWidget)
  (Default|ShowWidget (Variables|Default|GetNarratorWidget))
  (CallFunction|ShowText)
  (CallFunction|HandleNextText))

(fn StopTalking
  (bind _narratorwidget (Variables|Default|GetNarratorWidget))
  (bind _talkerwidget (Variables|Default|GetTalkerWidget))
  (if (Variables|Default|GetbNarrator)
    (Default|HideWidget _narratorwidget)
    (Default|ClearText _narratorwidget)
    (EventDispatchers|UnbindallEventsfromUserRequestNext _narratorwidget)
    (else
      (Class|BPITextBoxInterface|HideWidget(Message) _talkerwidget)
      (Class|BPITextBoxInterface|ClearText(Message) _talkerwidget)
      (EventDispatchers|UnbindallEventsfromUserRequestNext _talkerwidget)
      (Class|BPITalkerManagerInterface|ReleaseTextBox(Message) (Variables|Default|GetTalkerManager) _talkerwidget))))

(fn NextLine
  (CallFunction|ShowText)
  (CallFunction|HandleNextText))

(fn HandleNextText
  (bind _returnvalue (Class|DialogueComponent|GetCurrentText))
  (bind _timer (Utilities|Struct|BreakDialogueData _returnvalue))
  (if (> _timer 0.0)
    (bind _returnvalue_2 (Utilities|Time|SetTimerbyEvent (EventDispatchers|CreateEvent :!event Next) _timer))
    (Variables|Default|SetNextLineTimer _returnvalue_2)))

(fn InitializeWidget
  (if (Variables|Default|GetbNarrator)
    (bind _foundwidgets (Widget|GetAllWidgetsOfClass "/Game/Blueprints/UI/Text/WBP_NarratorSubtitleTextBox.WBP_NarratorSubtitleTextBox_C" false))
    (Variables|Default|SetNarratorWidget (Utilities|Array|Get(acopy) _foundwidgets))
    (elif (not (Utilities|IsValid (Variables|Default|GetTalkerWidget)))
      (if (Utilities|IsValid (Variables|Default|GetTalkerManager))
        _
        (else
          (bind _foundwidgets_2 (Widget|GetAllWidgetsOfClass "/Game/Blueprints/UI/Text/WBP_TalkerManager.WBP_TalkerManager_C" false))
          (Variables|Default|SetTalkerManager (Utilities|Array|Get(acopy) _foundwidgets_2))))
      (bind _freewidget (Class|BPITalkerManagerInterface|GetTextBox(Message) (Variables|Default|GetTalkerManager)))
      (Variables|Default|SetTalkerWidget _freewidget))))

(fn ShowText
  (bind _returnvalue (Class|DialogueComponent|GetCurrentText))
  (bind _line (Utilities|Struct|BreakDialogueData _returnvalue))
  (if (Variables|Default|GetbNarrator)
    (Default|SetText (Variables|Default|GetNarratorWidget) _line)
    (else
      (Default|SetText (Variables|Default|GetTalkerWidget) _line))))

(fn TestText
  (bind _returnvalue (Class|DialogueComponent|InitializeText "A" 3.0))
  (bind _returnvalue_2 (Class|DialogueComponent|AddLine _returnvalue "B" 3.0))
  (bind _returnvalue_3 (Class|DialogueComponent|AddLine _returnvalue_2 "C" 3.0))
  (Utilities|FlowControl|Sequence
    (:then_0
      (bind _returnvalue_4 (Class|DialogueComponent|AddBranch _returnvalue_3 (Utilities|Struct|MakeBranchInput 2 "D") 3.0))
      (bind _returnvalue_5 (Class|DialogueComponent|AddLine _returnvalue_4 "E" 3.0))
      (Class|DialogueComponent|AddLine _returnvalue_5 "F" 3.0))
    (:then_1
      (bind _returnvalue_6 (Class|DialogueComponent|AddBranch _returnvalue_3 (Utilities|Struct|MakeBranchInput 1 "G") 3.0))
      (Class|DialogueComponent|AddLine _returnvalue_6 "H" 3.0))))

(fn HideTemporary
  (bind _narratorwidget (Variables|Default|GetNarratorWidget))
  (bind _talkerwidget (Variables|Default|GetTalkerWidget))
  (if (Variables|Default|GetbNarrator)
    (Default|HideWidget _narratorwidget)
    (Default|ClearText _narratorwidget)
    (else
      (Class|BPITextBoxInterface|HideWidget(Message) _talkerwidget)
      (Class|BPITextBoxInterface|ClearText(Message) _talkerwidget))))