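; BP_MemoryPuzzle is a memory-matching puzzle piece that hides and reveals itself behind a sliding curtain.
; On BeginPlay it sets the BPACMemory component's text state to Memory and displays that on its text render.
; RevealObject and HideObject use timelines to nudge the curtain in opposite local X directions on each update.
; StayRevealed flags both the compared object and its own memory component as completed; MatchedObject is an empty stub.
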(event Custom|HideObject
  (Timeline|Timeline_1 PlayFromStart
    (:Update
      (Transformation|AddLocalOffset (Variables|Default|GetCurtain) "2.500000,0.000000,0.000000" false false))))

(event Custom|StayRevealed
  (params (ComparedObject :type BPAC%20Memory%20Object%20Object%20Reference))
  (Variables|/Game/Blueprints/BPAC_MemoryObject.BPAC_MemoryObject_C|SetCompleted ComparedObject true)
  (Variables|/Game/Blueprints/BPAC_MemoryObject.BPAC_MemoryObject_C|SetCompleted (Variables|Default|GetBPAC_Memory) true))

(event Custom|RevealObject
  (params (ComparedObject :type BPAC%20Memory%20Object%20Object%20Reference))
  (Timeline|Timeline_0 PlayFromStart
    (:Update
      (Transformation|AddLocalOffset (Variables|Default|GetCurtain) "-2.500000,0.000000,0.000000" false false))))

(event EventBeginPlay
  (bind _output_get (Variables|/Game/Blueprints/BPAC_MemoryObject.BPAC_MemoryObject_C|SetTextState (Variables|Default|GetBPAC_Memory) (Variables|Default|GetMemory)))
  (Rendering|Components|TextRender|SetText (Variables|Default|GetTextRender) (Utilities|Text|ToText(String) (Utilities|String|EnumtoString _output_get))))

(fn ConstructionScript)

(fn MatchedObject)