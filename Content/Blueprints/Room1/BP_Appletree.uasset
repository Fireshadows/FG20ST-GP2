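; BP_Appletree is a Room1 puzzle tree whose apples cannot be dragged until a ladder is snapped to it.
; BeginPlay locks every apple in the Apples array and prints an out-of-reach message when one is grabbed.
; When an actor whose BPAC_Snappable targets this tree overlaps TreeHitbox, it attaches to LadderSocket, stops being draggable and unlocks the apples.
; Older snap and detach logic remains disconnected.
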(event OnComponentBeginOverlap(TreeHitbox)
  (params (OverlappedComponent :type Primitive%20Component%20Object%20Reference) (OtherActor :type Actor%20Object%20Reference) (OtherComp :type Primitive%20Component%20Object%20Reference) (OtherBodyIndex :type Integer) (bFromSweep :type Boolean) (SweepResult :type Hit%20Result%20Structure%20%28by%20ref%29))
  (bind _returnvalue (Components|GetOwner OtherComp))
  (bind _returnvalue_2 (Actor|GetComponentbyClass _returnvalue "/Game/Blueprints/BPAC_Snappable.BPAC_Snappable_C"))
  (bind _returnvalue_3 (Actor|GetComponentbyClass _returnvalue "/Game/Blueprints/BPAC_Draggable.BPAC_Draggable_C"))
  (if (Utilities|IsValid OtherComp)
    (if (and (Utilities|IsValid _returnvalue_2) (== (Variables|/Game/Blueprints/BPAC_Snappable.BPAC_Snappable_C|GetTargetActor _returnvalue_2) self))
      (Utilities|IsValid (Variables|Default|GetSnappedActor)
        (:Is%20Not%20Valid
          (Transformation|AttachActorToActor _returnvalue self "LadderSocket" "SnapToTarget" "SnapToTarget" "SnapToTarget" true)
          (Variables|Default|SetSnappedActor _returnvalue)
          (if (Utilities|IsValid _returnvalue_3)
            (Variables|/Script/FGGP2.InteractBaseComponent|Setinteractable _returnvalue_3 false)
            (CallFunction|SetChildInteractability true)))))))

(event Custom|OnGrabbingUnavailableApple
  (Development|PrintString "Cannot reach these apples!"))

(event EventBeginPlay
  (CallFunction|SetChildInteractability false)
  (for _array_element (Variables|Default|GetApples)
    (if (Utilities|IsValid (Actor|GetComponentbyClass _array_element "/Game/Blueprints/BPAC_Draggable.BPAC_Draggable_C"))
      (EventDispatchers|BindEventtoOnDragUninteractable (Actor|GetComponentbyClass _array_element "/Game/Blueprints/BPAC_Draggable.BPAC_Draggable_C") (delegate Custom|OnGrabbingUnavailableApple)))))

(event EventTick
  (params (DeltaSeconds :type Float%20%28single-precision%29)))

(fn ConstructionScript)

(fn SetChildInteractability
  (params (Become%20Interactable :type Boolean))
  (for _array_element (Variables|Default|GetApples)
    (bind _asbp_apple (Utilities|Casting|CastToBP_Apple _array_element))
    (Variables|/Script/FGGP2.InteractBaseComponent|Setinteractable (Actor|GetComponentbyClass _asbp_apple "/Game/Blueprints/BPAC_Draggable.BPAC_Draggable_C") Become%20Interactable)))