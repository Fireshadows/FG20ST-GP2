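; BP_Rotating is an actor that continually turns to face a camera, billboard style.
; On BeginPlay it calls GetCameraMessage on player 0's view target and caches the returned camera.
; Each Tick it sets its rotation to look from its own location toward that camera's CameraComponent.
; The camera reference is not refreshed afterward, so later view target changes are not followed.
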(event EventTick
  (params (DeltaSeconds :type Float%20%28single-precision%29))
  (Transformation|SetActorRotation (Math|Rotator|FindLookatRotation (Transformation|GetActorLocation) (Transformation|GetWorldLocation (Variables|/Script/Engine.CameraActor|GetCameraComponent (Variables|Default|GetCamera))))))

(event EventBeginPlay
  (bind _camera (Class|BPICamera|GetCamera(Message) (Pawn|GetViewTarget (Game|GetPlayerController 0))))
  (Variables|Default|SetCamera _camera))

(fn ConstructionScript)