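; BPAC_Interactable is an actor component that lets its owning actor respond to click and drag interactions.
; The Clickable and Draggable events are each gated by a shared Interactable flag plus their own Click or Drag flag.
; Clicking only prints a debug message, while dragging also moves the owner to the supplied location's X and Y, keeping its current Z, without sweep.
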(event EventClickable
  (if (Variables|Default|GetInteractable)
    (if (Variables|Default|GetClick)
      (Development|PrintString "Click"))))

(event EventDraggable
  (params (;ouse%20Location :type Vector :default "0, 0, 0"))
  (bind _returnvalue (Components|GetOwner))
  (bind (_x _y) (Math|Vector|BreakVector ;ouse%20Location))
  (if (Variables|Default|GetInteractable)
    (if (Variables|Default|GetDrag)
      (Development|PrintString "Drag")
      (Transformation|SetActorLocation _returnvalue (Math|Vector|MakeVector _x _y (.Z (Math|Vector|BreakVector (Transformation|GetActorLocation _returnvalue)))) false false))))