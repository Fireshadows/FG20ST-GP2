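; BPAC_Storable is an actor component that lets the player pick up its owning actor into inventory.
; On Click, if Interactable, it clears the flag, hides the owner and passes it to the player pawn through InventoryMessage.
; The component does not store the item itself, leaving that to whatever handles the message on the pawn.
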(event EventClick
  (if (Variables|Default|GetInteractable)
    (bind _output_get (Variables|Default|SetInteractable (not (Variables|Default|GetInteractable))))
    (Rendering|SetActorHiddenInGame (Components|GetOwner) (not _output_get))
    (Class|BPInventoryInterface|Inventory(Message) (Game|Player|GetPlayerPawn 0) (Components|GetOwner))))

(event EventBeginPlay)