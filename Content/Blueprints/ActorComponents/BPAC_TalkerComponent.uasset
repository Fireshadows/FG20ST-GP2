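; Actor component that lets its owning actor talk through on-screen subtitle text boxes, starting or advancing when clicked.
; It responds to started, next and finished subtitle events by borrowing a text box from WBP_TalkerManager, showing each line with optional 2D sound, then releasing it.
; Fixed-duration lines auto-advance by timer.
; While talking, Tick projects the owner's location to screen space so the box follows it.
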(event EventBeginPlay
  (Utilities|FlowControl|Delay 0.2)
  (CallFunction|SetTalkerManagerReference)
  (|SubtitleEventBinding))

(event EventTick
  (params (DeltaSeconds :type Float%20%28single-precision%29))
  (bind _currentlyusedtextbox (Variables|Default|GetCurrentlyUsedTextBox))
  (if (not (Variables|Default|GetFinishedTalking?))
    (if (Variables|Default|GetbHasStarted)
      (Utilities|IsValid _currentlyusedtextbox
        (:Is%20Valid
          (bind (_viewport_position _actorinviewport_) (CallFunction|GetActorLocationinViewport (Components|GetOwner)))
          (if _actorinviewport_
            (Default|SetPosition _currentlyusedtextbox _viewport_position)))))))

(event EventClickable
  (if (Variables|Default|Getinteractable)
    (if (not (Variables|Default|GetFinishedTalking?))
      (if (Variables|Default|GetbHasStarted)
        (Class|SubtitleComponent|Clicked)
        (else
          (Class|SubtitleComponent|Start))))))

(fn ManageSubtitleEventImpl
  (params (SubtitleEvent :type ESubtitleEvent%20Enum :default "SubtitleFinished"))
  (switch Utilities|FlowControl|Switch|SwitchonESubtitleEvent SubtitleEvent
    (:SubtitleFinished
      (CallFunction|StopShowingText)
      (Default|CallFinishedTalking)
      (Variables|Default|SetFinishedTalking? true))
    (:SubtitleStarted
      (CallFunction|StartShowingText))
    (:SubtitleNext
      (CallFunction|NewTexttoShow))))

(fn SetTalkerManagerReference
  (bind _foundwidgets (Widget|GetAllWidgetsOfClass "/Game/Blueprints/UI/Text/WBP_TalkerManager.WBP_TalkerManager_C" false))
  (Variables|Default|SetTalkerManager (Utilities|Array|Get(acopy) _foundwidgets)))

(fn StartShowingText
  (if (Utilities|IsValid (Variables|Default|GetCurrentlyUsedTextBox))
    _
    (else
      (bind _freewidget (Default|GetTextBox (Variables|Default|GetTalkerManager)))
      (Variables|Default|SetCurrentlyUsedTextBox _freewidget)))
  (Class|BPITextBoxInterface|ShowWidget(Message) (Variables|Default|GetCurrentlyUsedTextBox))
  (CallFunction|ShowTextImpl)
  (CallFunction|HandleNextText))

(fn StopShowingText
  (if (Utilities|IsValid (Variables|Default|GetCurrentlyUsedTextBox))
    (Default|ReleaseTextBox (Variables|Default|GetTalkerManager) (Variables|Default|GetCurrentlyUsedTextBox))))

(fn HandleNextText
  (bind _returnvalue (Class|SubtitleComponent|GetCurrentTextData))
  (switch Utilities|FlowControl|Switch|SwitchonENextLineTrigger (.triggerType (Utilities|Struct|BreakTextData _returnvalue))
    (:OnFixedDuration
      (Utilities|Time|SetTimerbyFunctionName 0 "Next" (.duration (Utilities|Struct|BreakTextData _returnvalue))))))

(fn GetActorLocationinViewport
  (params (Actor :type Actor%20Object%20Reference))
  (bind _returnvalue (Game|GetPlayerController 0))
  (bind _returnvalue_2 (Transformation|GetActorLocation Actor))
  (bind (_screenposition _returnvalue_3) (Class|WidgetLayoutLibrary|ProjectWorldLocationtoWidgetPosition _returnvalue _returnvalue_2 false))
  (return _screenposition _returnvalue_3))

(fn ShowTextImpl
  (bind _returnvalue (Class|SubtitleComponent|GetCurrentTextData))
  (Class|BPITextBoxInterface|SetText(Message) (Variables|Default|GetCurrentlyUsedTextBox) (.line (Utilities|Struct|BreakTextData _returnvalue)))
  (if (Utilities|IsValid (.soundRef (Utilities|Struct|BreakTextData _returnvalue)))
    (Audio|PlaySound2D (.soundRef (Utilities|Struct|BreakTextData _returnvalue)) 1.0 1.0 0.0 0 0))
  (bind _viewport_position (CallFunction|GetActorLocationinViewport (Components|GetOwner)))
  (Class|BPITextBoxInterface|SetPosition(Message) (Variables|Default|GetCurrentlyUsedTextBox) _viewport_position)
  (return))

(fn NewTexttoShow
  (CallFunction|ShowTextImpl)
  (CallFunction|HandleNextText))

(event Custom|ManageSubtitles
  (params (SubtitleEvent :type ESubtitleEvent%20Enum :default "SubtitleFinished"))
  (CallFunction|ManageSubtitleEventImpl SubtitleEvent))