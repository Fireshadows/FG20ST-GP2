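; Actor component that lets its owner be clicked into the player's inventory and taken back out.
; Clickable checks inventory space, then toggles the stored state, hiding the actor, and notifies the player pawn.
; Retrieval comes from the inventory element widget; unstoring a BPAC_Draggable owner hands it straight to BP_Character as an active drag.
; Draggable owners are repositioned at opposite X offsets from the camera when stored and retrieved.
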(event EventClickable
  (bind _returnvalue (Game|Player|GetPlayerPawn 0))
  (bind _returnvalue_2 (Components|GetOwner))
  (bind _returnvalue_3 (Actor|GetComponentbyClass _returnvalue_2 "/Game/Blueprints/ActorComponents/BPAC_Draggable.BPAC_Draggable_C"))
  (bind _originlocation (Variables|/Game/Blueprints/ActorComponents/BPAC_Draggable.BPAC_Draggable_C|GetOriginLocation _returnvalue_3))
  (bind (_x _y _z) (Math|Vector|BreakVector _originlocation))
  (bind _returnvalue_4 (Class|Inventory|IsNotFull (Actor|GetComponentbyClass _returnvalue "/Script/FGGP2.Inventory")))
  (if _returnvalue_4
    (if (Variables|Default|GetInteractable)
      (if (not (Variables|Default|GetStored))
        ;[1 1 1] This code is executed for items that gets stored
        (CallFunction|ToggleStoreState)
        (Class|BPInventoryInterface|Inventory(Message) _returnvalue _returnvalue_2)
        (Utilities|IsValid _returnvalue_3
          (:Is%20Valid
            (Transformation|SetActorLocation (Components|GetOwner) (Math|Vector|MakeVector (- (.X (Math|Vector|BreakVector (Camera|GetCameraLocation (Game|GetPlayerCameraManager 0)))) (Variables|Default|GetInventoryObjectOffset)) _y _z) false false)))
        (else
          ;[1 1 1] The code for items that gets taken out from an inventory is located in inventoryelement widget
          (Development|PrintString "Is already Stored" true true "(R=1.000000,G=0.062500,B=0.062500,A=1.000000)")))
      (else
        (Development|PrintString "Not interactable" true true "(R=1.000000,G=0.062500,B=0.062500,A=1.000000)")))
    (else
      (Development|PrintString "Cannot Add More" true true "(R=1.000000,G=0.062500,B=0.062500,A=1.000000)"))))

(fn ToggleStoreState
  (bind _returnvalue (Components|GetOwner))
  (bind _returnvalue_2 (Components|GetOwner))
  (bind _returnvalue_3 (Transformation|GetActorLocation _returnvalue))
  (bind _returnvalue_4 (Actor|GetComponentbyClass _returnvalue_2 "/Game/Blueprints/ActorComponents/BPAC_Draggable.BPAC_Draggable_C"))
  (bind (_x _y _z) (Math|Vector|BreakVector _returnvalue_3))
  (bind _output_get (Variables|Default|SetStored (not (Variables|Default|GetStored))))
  (bind _output_get_2 (Variables|Default|SetInteractable (not _output_get)))
  (Rendering|SetActorHiddenInGame (Components|GetOwner) (not _output_get_2))
  (if (not (Variables|Default|GetStored))
    (if (Utilities|IsValid _returnvalue_4)
      (Variables|/Script/FGGP2.InteractBaseComponent|Setinteractable _returnvalue_4 true)
      (bind _asbp_character (Utilities|Casting|CastToBP_Character (Game|Player|GetPlayerPawn 0)))
      (bind _output_get_3 (Variables|/Game/Blueprints/Core/BP_Character.BP_Character_C|SetDraggingComponent _asbp_character _returnvalue_4))
      (Variables|/Game/Blueprints/Core/BP_Character.BP_Character_C|SetIsDragging? _asbp_character true)
      (Variables|/Game/Blueprints/Core/BP_Character.BP_Character_C|SetMouseClicked _asbp_character true)
      (Transformation|SetActorLocation _returnvalue (Math|Vector|MakeVector (+ (.X (Math|Vector|BreakVector (Camera|GetCameraLocation (Game|GetPlayerCameraManager 0)))) (Variables|Default|GetInventoryObjectOffset)) _y _z) false false))))