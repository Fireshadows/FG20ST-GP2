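; Actor component that lets the player mouse-drag its owner along the Y/Z plane and drop it onto receiving actors.
; Draggable projects the cursor at the owner's distance, applies axis locks, offset and optional interpolation, then clamps to room bounds from BP_Gamestate.
; Tick re-arms the once-per-click interactable events on mouse release.
; StopDragging traces under the cursor, offers the owner via ReceiveItemMessage, and can return it to origin if none accepts.
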(event EventStartDragging
  (Default|CallStartedDragging))

(event EventStopDragging
  (bind _returnvalue (Game|GetPlayerController 0))
  (bind (_worldlocation _worlddirection) (Game|Player|ConvertMouseLocationToWorldSpace _returnvalue))
  (bind _returnvalue_2 (* _worlddirection 2e+03))
  (bind _returnvalue_3 (+ _worldlocation _returnvalue_2))
  (Default|CallStoppedDragging)
  (if (Variables|Default|Getinteractable)
    (Rendering|Debug|DrawDebugLine _worldlocation _returnvalue_3 "(R=0.000000,G=0.000000,B=0.000000,A=1.000000)" 1e+01 0.0)
    (bind (_outhits _returnvalue_4) (Class|KismetSystemLibrary|LineTraceMultiforObjects _worldlocation _returnvalue_3 (Utilities|Array|MakeArray "ObjectTypeQuery1" "ObjectTypeQuery2") true 0 "None" true))
    (if _returnvalue_4
      (bind _array_element (Utilities|Array|ForEachLoopwithBreak _outhits :!label _label)
        (:LoopBody
          (bind _wasitemconsumed_ (Class|BPIItemInteractableInterface|ReceiveItem(Message) (.HitActor (Collision|BreakHitResult _array_element)) (Components|GetOwner self) (.HitComponent (Collision|BreakHitResult _array_element))))
          (if _wasitemconsumed_
            (Variables|Default|SetbDidCollide true)
            (goto _label Break)))
        (:Completed
          (if (and (not (Variables|Default|GetbDidCollide)) (Variables|Default|GetGoToOriginOnEndDrag)) :!label _label_2
            (Transformation|SetActorLocation (Components|GetOwner) (Variables|Default|GetOriginLocation) false false))))
      (else
        (goto _label_2)))))

(event EventTick
  (params (DeltaSeconds :type Float%20%28single-precision%29))
  (Variables|Interpolation|SetDelta DeltaSeconds)
  (Utilities|FlowControl|Sequence
    (:then_0
      (if (Variables|Default|GetInteractableEventClosed)
        (if (not (Variables|/Game/Blueprints/Core/BP_Character.BP_Character_C|GetMouseClicked (Variables|Default|GetCharacter)))
          (Variables|Default|SetInteractableEventClosed false)
          (Utilities|FlowControl|DoOnce false) ; enters at Reset
        )))
    (:then_1
      (if (Variables|Default|GetUninteractableEventClosed)
        (if (not (Variables|/Game/Blueprints/Core/BP_Character.BP_Character_C|GetMouseClicked (Variables|Default|GetCharacter)))
          (Variables|Default|SetUninteractableEventClosed false)
          (Utilities|FlowControl|DoOnce false) ; enters at Reset
        )))))

(event EventDraggable
  (bind _returnvalue (Components|GetOwner))
  (bind _drag_interp_speed (Variables|Interpolation|GetDrag%20Interp%20Speed))
  (bind _delta (Variables|Interpolation|GetDelta))
  (bind _returnvalue_2 (Transformation|GetActorLocation _returnvalue))
  (if (Variables|Default|Getinteractable)
    (Utilities|FlowControl|Sequence
      (:then_0
        (bind _newparam (CallFunction|GetNewPosition))
        (if (Variables|Interpolation|GetInterpolate)
          (if (Variables|Interpolation|GetSmooth%20Interpolation)
            (Variables|Default|SetNewLocation (Math|Interpolation|VInterpTo _returnvalue_2 _newparam _delta _drag_interp_speed))
            (else
              (Variables|Default|SetNewLocation (Math|Interpolation|VInterptoConstant _returnvalue_2 _newparam _delta (* 1e+02 _drag_interp_speed)))))
          (else
            (Variables|Default|SetNewLocation _newparam)))
        (Transformation|SetActorLocation _returnvalue (Variables|Default|GetNewLocation) false false)
        (CallFunction|CheckBoundaries)
        (Default|CallDragging (Variables|Default|GetRawLocation)))
      (:then_1
        (Utilities|FlowControl|DoOnce false
          (:Completed
            (Default|CallOnDragInteractable)
            (Variables|Default|SetInteractableEventClosed true)))))
    (else
      (Utilities|FlowControl|DoOnce false
        (:Completed
          (Default|CallOnDragUninteractable)
          (Variables|Default|SetUninteractableEventClosed true))))))

(event EventBeginPlay
  (bind _asbp_character (Utilities|Casting|CastToBP_Character (Game|Player|GetPlayerPawn 0)))
  (Variables|Default|SetCharacter _asbp_character)
  (Variables|Default|SetOriginLocation (Transformation|GetActorLocation (Components|GetOwner)))
  (bind _asbp_gamestate (Utilities|Casting|CastToBP_Gamestate (Game|GetGameState)))
  (Variables|Default|SetGameState _asbp_gamestate))

(fn GetNewPosition
  (bind _returnvalue (Game|GetPlayerController 0))
  (bind _returnvalue_2 (Components|GetOwner))
  (bind _returnvalue_3 (Components|GetOwner))
  (bind _dragoffset (Variables|Default|GetDragOffset))
  (bind _lock_vertical (Variables|Default|GetLock%20Vertical))
  (bind (_worldlocation _worlddirection) (Game|Player|ConvertMouseLocationToWorldSpace _returnvalue))
  (bind _returnvalue_4 (Transformation|GetActorLocation _returnvalue_2))
  (bind _returnvalue_5 (Transformation|GetActorLocation _returnvalue_3))
  (bind _returnvalue_6 (Math|Vector|Distance(Vector) _returnvalue_5 _worldlocation))
  (bind (_x _y _z) (Math|Vector|BreakVector _returnvalue_4))
  (bind _returnvalue_7 (Math|Vector|Normalize _worlddirection))
  (bind _returnvalue_8 (* _returnvalue_7 _returnvalue_6))
  (bind _returnvalue_9 (+ _worldlocation _returnvalue_8))
  (bind (_x_2 _y_2 _z_2) (Math|Vector|BreakVector _returnvalue_9))
  (bind _output_get (LocalVariables|Setresult (Math|Vector|MakeVector (.X (Math|Vector|BreakVector _returnvalue_5)) _y_2 _z_2)))
  (Variables|Default|SetRawLocation _output_get)
  (if _lock_vertical
    (LocalVariables|Setresult (- (Math|Vector|MakeVector (.X (Math|Vector|BreakVector (LocalVariables|Getresult))) (.Y (Math|Vector|BreakVector (LocalVariables|Getresult))) _z) (Math|Vector|MakeVector 0.0 (.y (Variables|Default|GetDragOffset)) 0.0))))
  (if (Variables|Default|GetLock%20Horizontal)
    (LocalVariables|Setresult (- (Math|Vector|MakeVector (.X (Math|Vector|BreakVector (LocalVariables|Getresult))) _y (.Z (Math|Vector|BreakVector (LocalVariables|Getresult)))) (Math|Vector|MakeVector 0.0 0.0 (.z (Variables|Default|GetDragOffset)))))
    (elif _lock_vertical
      _
      (else
        (LocalVariables|Setresult (- (LocalVariables|Getresult) (Math|Vector|MakeVector 0.0 (.y _dragoffset) (.z _dragoffset)))))))
  (return (LocalVariables|Getresult)))

(fn OnSnappedinNewPosition
  (Variables|Default|Setinteractable false)
  (Variables|Default|SetGoToOriginOnEndDrag false)
  (bind _asstatic_mesh_actor (Utilities|Casting|CastToStaticMeshActor (Components|GetOwner)))
  (Collision|SetCollisionResponsetoChannel (Variables|/Script/Engine.StaticMeshActor|GetStaticMeshComponent _asstatic_mesh_actor) "ECC_Visibility" "ECR_Ignore"))

(fn CheckBoundaries
  (bind _returnvalue (Components|GetOwner))
  (bind _returnvalue_2 (Components|GetOwner))
  (bind _gamestate (Variables|Default|GetGameState))
  (bind _returnvalue_3 (Transformation|GetActorLocation _returnvalue_2))
  (bind _returnvalue_4 (Transformation|GetActorLocation _returnvalue))
  (bind _roomdimensions (Variables|/Game/Blueprints/Core/BP_Gamestate.BP_Gamestate_C|GetRoomDimensions _gamestate))
  (bind _maincamera (Variables|/Game/Blueprints/Core/BP_Gamestate.BP_Gamestate_C|GetMainCamera _gamestate))
  (bind _returnvalue_5 (Transformation|GetActorLocation _maincamera))
  (bind (_x _y _z) (Math|Vector|BreakVector _returnvalue_3))
  (Utilities|IsValid _returnvalue_2
    (:Is%20Valid
      (bind _floor_value (Default|GetFloorOfRoom (Variables|Default|GetGameState)))
      (if (> _floor_value _z)
        (Transformation|SetActorLocation (Components|GetOwner) (Math|Vector|MakeVector _x _y _floor_value) false false))
      (LocalVariables|SetDepthBoundaries (Math|Vector2D|MakeVector2D (- (.x _returnvalue_5) (.x _roomdimensions)) (+ (.x _roomdimensions) (.x _returnvalue_5))))
      (LocalVariables|SetHorizontalBoundaries (Math|Vector2D|MakeVector2D (- (.y _returnvalue_5) (.y _roomdimensions)) (+ (.y _roomdimensions) (.y _returnvalue_5))))
      (LocalVariables|SetVerticalBoundaries (Math|Vector2D|MakeVector2D (- (.z _returnvalue_5) (.z _roomdimensions)) (+ (.z _roomdimensions) (.z _returnvalue_5))))
      (LocalVariables|SetX (.x _returnvalue_4))
      (LocalVariables|SetY (.y _returnvalue_4))
      (LocalVariables|SetZ (.z _returnvalue_4))
      (bind _clamped_value (CallFunction|ClampValue (LocalVariables|GetY) (LocalVariables|GetHorizontalBoundaries)))
      (LocalVariables|SetY _clamped_value)
      (bind _clamped_value_2 (CallFunction|ClampValue (LocalVariables|GetZ) (LocalVariables|GetVerticalBoundaries)))
      (LocalVariables|SetZ _clamped_value_2)
      (Transformation|SetActorLocation (Components|GetOwner) (Math|Vector|MakeVector (LocalVariables|GetX) (LocalVariables|GetY) (LocalVariables|GetZ)) false false))))

(fn ClampValue
  (params (Value :type Float%20%28single-precision%29) (Clamps :type Vector%202D%20Structure))
  (bind (_x _y) (Math|Vector2D|BreakVector2D Clamps))
  (LocalVariables|SetClamped Value)
  (if (< (LocalVariables|GetClamped) _x)
    (LocalVariables|SetClamped _x)
    (elif (> (LocalVariables|GetClamped) _y)
      (LocalVariables|SetClamped _y)))
  (return (LocalVariables|GetClamped)))