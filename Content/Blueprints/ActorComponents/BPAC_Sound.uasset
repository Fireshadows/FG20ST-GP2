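; BPAC_Sound is an actor component that plays a configurable sound for click and drag interactions.
; Its Clickable and Draggable events each play the sound at the world origin, then call Clicked or Dragged respectively.
; Each event has its own DoOnce that resets after a Timer delay, throttling repeat triggers independently.
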(event EventClickable
  (Utilities|FlowControl|DoOnce false :!label _label
    (:Completed
      (Audio|PlaySoundatLocation (Variables|Default|GetSound) "0, 0, 0" "0, 0, 0" 1.0 1.0 0.0 0 0 0)
      (Default|CallClicked)
      (Utilities|FlowControl|Delay (Variables|Default|GetTimer))
      (goto _label Reset))))

(event EventDraggable
  (Utilities|FlowControl|DoOnce false :!label _label
    (:Completed
      (Audio|PlaySoundatLocation (Variables|Default|GetSound) "0, 0, 0" "0, 0, 0" 1.0 1.0 0.0 0 0 0)
      (Default|CallDragged)
      (Utilities|FlowControl|Delay (Variables|Default|GetTimer))
      (goto _label Reset))))