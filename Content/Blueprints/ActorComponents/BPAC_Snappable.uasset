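; Actor component meant to make its owner snap to a target actor when dragged, currently an unfinished stub with no snapping logic.
; On BeginPlay it prints a warning if the target actor is unset, then binds to the drag event of the owner's BPAC_Draggable.
; The drag handler is empty, and disconnected nodes hold a debug print and code to make a static mesh owner ignore the Visibility channel.
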(event Custom|OnDraggingSnappable
  ;[1 1 1] Not tied to anything! /Lee
)

(event EventBeginPlay
  (if (Utilities|IsValid (Variables|Default|GetTargetActor))
    _
    (else
      (Development|PrintString (Utilities|String|Append (Utilities|GetObjectName self) " is missing a target actor to snap to") true true "(R=0.000000,G=0.000000,B=0.000000,A=1.000000)" 5.0)))
  (EventDispatchers|BindEventtoOnDragInteractable (Actor|GetComponentbyClass (Components|GetOwner) "/Game/Blueprints/ActorComponents/BPAC_Draggable.BPAC_Draggable_C") (delegate Custom|OnDraggingSnappable)))