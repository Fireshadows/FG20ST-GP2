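; Narrator actor component that presents a data asset's lines as subtitles with optional sound, labelled with the owning actor's name.
; It finds the existing subtitle widget after a short delay, then reacts to Started, Next and Finished subtitle events.
; Each line's trigger type decides timed or click advancing, using inherited timer and click logic.
; ShowText and NextTextTimerTriggered form a separate timer-by-name playback path that the event graph never calls.
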(event Custom|Finished
  (Default|HideWidget (Variables|Default|GetNarratorTextBox))
  (Class|SubtitleComponent|StopTimer))

(event Custom|ManageSubtitles
  (params (SubtitleEvent :type ESubtitleEvent%20Enum :default "SubtitleFinished"))
  (bind _narratortextbox (Variables|Default|GetNarratorTextBox))
  (switch Utilities|FlowControl|Switch|SwitchonESubtitleEvent SubtitleEvent
    (:SubtitleFinished
      (Variables|Default|SetFinishedTalking? true)
      (Default|CallNarratorFinished))
    (:SubtitleStarted
      (Class|BPITextBoxInterface|ShowWidget(Message) _narratortextbox)
      (CallFunction|ShowTextImpl)
      (CallFunction|HandleNextText)
      (Default|ShowNextButton _narratortextbox :!label _label))
    (:SubtitleNext
      (CallFunction|ShowTextImpl)
      (CallFunction|HandleNextText)
      (goto _label))))

(event Custom|UserRequestNext
  (Class|SubtitleComponent|Clicked))

(event EventBeginPlay
  (Utilities|FlowControl|Delay 0.5)
  (bind _foundwidgets (Widget|GetAllWidgetsOfClass "/Game/Blueprints/UI/Text/WBP_NarratorSubtitleTextBox.WBP_NarratorSubtitleTextBox_C" false))
  (if (> (Utilities|Array|Length _foundwidgets) 0)
    (bind _output_get (Variables|Default|SetNarratorTextBox (Utilities|Array|Get(acopy) _foundwidgets)))
    (EventDispatchers|BindEventtoUserRequestNext _output_get (delegate Custom|UserRequestNext))
    (EventDispatchers|BindEventtoNarratorFinished (delegate Custom|Finished))
    (EventDispatchers|BindEventtoSubtitleEvent (delegate Custom|ManageSubtitles))))

(event EventTick
  (params (DeltaSeconds :type Float%20%28single-precision%29)))

(event EventClickable
  (if (Variables|Default|Getinteractable)
    (if (not (Variables|Default|GetFinishedTalking?))
      (if (Variables|Default|GetbHasStarted)
        (bind _returnvalue (Class|SubtitleComponent|GetCurrentTextData))
        (switch Utilities|FlowControl|Switch|SwitchonENextLineTrigger (.triggerType (Utilities|Struct|BreakTextData _returnvalue))
          (:OnClick
            _)
          (:OnFixedDurationOrClick
            _)))
      (Class|SubtitleComponent|Clicked))))

(fn ShowText
  (bind _narratortextbox (Variables|Default|GetNarratorTextBox))
  (bind _dataasset (Variables|Default|GetDataAsset))
  (bind _currentline (Variables|Default|GetCurrentLine))
  (bind _texts (Variables|/Script/FGGP2.SubtitleDataAsset|Gettexts _dataasset))
  (bind _output (Utilities|Array|Get(acopy) _texts _currentline))
  (bind (_line _duration _triggertype _soundref) (Utilities|Struct|BreakTextData _output))
  (Default|ShowWidget _narratortextbox)
  (Default|SetText _narratortextbox _line)
  (Utilities|IsValid _soundref
    (:Is%20Valid
      (Audio|PlaySound2D _soundref 1.0 1.0 0.0 0 0))
    (:Is%20Not%20Valid
      _))
  (switch Utilities|FlowControl|Switch|SwitchonENextLineTrigger _triggertype
    (:OnClick
      _)
    (:OnFixedDuration
      (bind _returnvalue (Utilities|Time|SetTimerbyFunctionName 0 "NextTextTimerTriggered" _duration :!label _label))
      (Variables|Default|SetNextLineTimerHandle _returnvalue))
    (:OnFixedDurationOrClick
      (goto _label))
    (:OnTriggerEnter
      _))
  (return))

(fn NextTextTimerTriggered
  (bind _result (Math|Integer|IncrementInt (Variables|Default|GetCurrentLine))
    (:%20%20
      (if (< _result (Utilities|Array|Length (Variables|/Script/FGGP2.SubtitleDataAsset|Gettexts (Variables|Default|GetDataAsset))))
        (CallFunction|ShowText)
        (else
          (Default|CallNarratorFinished))))))

(fn ShowTextImpl
  (bind _narratortextbox (Variables|Default|GetNarratorTextBox))
  (bind _returnvalue (Class|SubtitleComponent|GetCurrentTextData))
  (Class|BPITextBoxInterface|SetText(Message) _narratortextbox (.line (Utilities|Struct|BreakTextData _returnvalue)))
  (if (Utilities|IsValid (.soundRef (Utilities|Struct|BreakTextData _returnvalue)))
    (Audio|PlaySound2D (.soundRef (Utilities|Struct|BreakTextData _returnvalue)) 1.0 1.0 0.0 0 0))
  (Default|SetName _narratortextbox (Utilities|String|StringToName (Utilities|GetObjectName (Components|GetOwner))))
  (return))

(fn HandleNextText
  (bind _returnvalue (Class|SubtitleComponent|GetCurrentTextData))
  (switch Utilities|FlowControl|Switch|SwitchonENextLineTrigger (.triggerType (Utilities|Struct|BreakTextData _returnvalue))
    (:OnFixedDuration
      _)
    (:OnFixedDurationOrClick
      _))
  (Class|SubtitleComponent|StartTimer (.duration (Utilities|Struct|BreakTextData _returnvalue))))