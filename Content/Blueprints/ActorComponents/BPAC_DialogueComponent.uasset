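; Actor component that plays an actor's dialogue lines, either in a shared narrator subtitle box named after the owner or in a talker text box that follows the actor on screen.
; Dialogue started, next and stopped events drive the widgets, with talker boxes borrowed from WBP_TalkerManager and released on stop.
; Lines advance on optional per-line timers, on skip requests when Skippable, or on clicks when Clickable, which also starts dialogue but ignores branch points.
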(event Custom|NextEvent
  (Utilities|Time|ClearandInvalidateTimerbyHandle (Variables|Default|GetNextLineTimer))
  (CallFunction|NextLine))

(event Custom|StartedEvent
  (CallFunction|StartTalking)
  (if (Variables|Default|GetbNarrator)
    (EventDispatchers|BindEventtoNarratorTextStarted (Variables|Default|GetNarratorWidget) (delegate Custom|AnimationStarted))
    (EventDispatchers|BindEventtoNarratorTextFinished (Variables|Default|GetNarratorWidget) (delegate Custom|AnimnationFinished))))

(event Custom|StoppedEvent
  (CallFunction|StopTalking)
  (Utilities|Time|ClearandInvalidateTimerbyHandle (Variables|Default|GetNextLineTimer))
  (if (Variables|Default|GetbNarrator)
    (EventDispatchers|UnbindallEventsfromNarratorTextFinished (Variables|Default|GetNarratorWidget))
    (EventDispatchers|UnbindallEventsfromNarratorTextStarted (Variables|Default|GetNarratorWidget))))

(event Custom|AnimationStarted
  (Default|CallAnimatedTextLineStarted))

(event Custom|AnimnationFinished
  (Default|CallAnimatedTextLineFinished))

(event EventBeginPlay
  (EventDispatchers|BindEventtoDialogueNext (delegate Custom|NextEvent))
  (EventDispatchers|BindEventtoDialogueStarted (delegate Custom|StartedEvent))
  (EventDispatchers|BindEventtoDialogueStopped (delegate Custom|StoppedEvent)))

(event EventTick
  (params (DeltaSeconds :type Float%20%28single-precision%29))
  (CallFunction|UpdateWidgetPosition))

(event EventClickable
  (if (Variables|Default|GetbClickable)
    (if (not (Class|DialogueComponent|AtBranch))
      (if (Variables|Default|GetbStarted)
        (Utilities|Time|ClearandInvalidateTimerbyHandle (Variables|Default|GetNextLineTimer))
        (Class|DialogueComponent|Next)
        (else
          (Class|DialogueComponent|Start))))))

(fn StartTalking
  (CallFunction|InitializeWidget)
  (CallFunction|ShowText)
  (CallFunction|HandleNextText))

(fn StopTalking
  (bind _narratorwidget (Variables|Default|GetNarratorWidget))
  (bind _talkerwidget (Variables|Default|GetTalkerWidget))
  (if (Variables|Default|GetbNarrator)
    (Default|HideWidget _narratorwidget)
    (Default|ClearText _narratorwidget)
    (EventDispatchers|UnbindallEventsfromUserRequestNext _narratorwidget)
    (else
      (Class|BPITextBoxInterface|HideWidget(Message) _talkerwidget)
      (Class|BPITextBoxInterface|ClearText(Message) _talkerwidget)
      (EventDispatchers|UnbindallEventsfromUserRequestNext _talkerwidget)
      (Class|BPITalkerManagerInterface|ReleaseTextBox(Message) (Variables|Default|GetTalkerManager) _talkerwidget))))

(fn NextLine
  (CallFunction|ShowText)
  (CallFunction|HandleNextText))

(fn HandleNextText
  (bind _returnvalue (Class|DialogueComponent|GetCurrentText))
  (bind _timer (Utilities|Struct|BreakDialogueData _returnvalue))
  (if (> _timer 0.0)
    (bind _returnvalue_2 (Utilities|Time|SetTimerbyEvent (EventDispatchers|CreateEvent :!event Next) _timer))
    (Variables|Default|SetNextLineTimer _returnvalue_2)))

(fn InitializeWidget
  (if (Variables|Default|GetbNarrator)
    (bind _foundwidgets (Widget|GetAllWidgetsOfClass "/Game/Blueprints/UI/Text/WBP_NarratorSubtitleTextBox.WBP_NarratorSubtitleTextBox_C" false))
    (bind _output_get (Variables|Default|SetNarratorWidget (Utilities|Array|Get(acopy) _foundwidgets)))
    (EventDispatchers|BindEventtoUserRequestNext _output_get (EventDispatchers|CreateEvent :!event UserRequestNext))
    (elif (not (Utilities|IsValid (Variables|Default|GetTalkerWidget)))
      (if (Utilities|IsValid (Variables|Default|GetTalkerManager))
        _
        (else
          (bind _foundwidgets_2 (Widget|GetAllWidgetsOfClass "/Game/Blueprints/UI/Text/WBP_TalkerManager.WBP_TalkerManager_C" false))
          (Variables|Default|SetTalkerManager (Utilities|Array|Get(acopy) _foundwidgets_2))))
      (bind _freewidget (Class|BPITalkerManagerInterface|GetTextBox(Message) (Variables|Default|GetTalkerManager)))
      (bind _output_get_2 (Variables|Default|SetTalkerWidget _freewidget))
      (EventDispatchers|BindEventtoUserRequestNext _output_get_2 (EventDispatchers|CreateEvent :!event UserRequestNext)))))

(fn ShowText
  (bind _returnvalue (Class|DialogueComponent|GetCurrentText))
  (bind _narratorwidget (Variables|Default|GetNarratorWidget))
  (bind _talkerwidget (Variables|Default|GetTalkerWidget))
  (bind _line (Utilities|Struct|BreakDialogueData _returnvalue))
  (if (Variables|Default|GetbNarrator)
    (Default|SetText _narratorwidget _line)
    (Class|BPITextBoxInterface|ShowWidget(Message) _narratorwidget)
    (Default|SetName _narratorwidget (Utilities|String|StringToName (Utilities|GetObjectName (Components|GetOwner))))
    (else
      (Default|SetText _talkerwidget _line)
      (Class|BPITextBoxInterface|ShowWidget(Message) _talkerwidget)
      (bind (_viewport_position _actorinviewport_) (CallFunction|GetActorLocationinViewport (Components|GetOwner)))
      (Class|BPITextBoxInterface|SetPosition(Message) _talkerwidget _viewport_position))))

(fn TestText
  (bind _returnvalue (Class|DialogueComponent|InitializeText "A" 3.0))
  (bind _returnvalue_2 (Class|DialogueComponent|AddLine _returnvalue "B" 3.0))
  (bind _returnvalue_3 (Class|DialogueComponent|AddLine _returnvalue_2 "C" 3.0))
  (bind _returnvalue_4 (Class|DialogueComponent|AddBranch _returnvalue_3))
  (Utilities|FlowControl|Sequence
    (:then_0
      (Class|DialogueComponent|AddLinetoBranch _returnvalue_4 (Utilities|Struct|MakeBranchInput 2 "D") 3.0)
      (bind _returnvalue_5 (Class|DialogueComponent|AddLine 0 "E" 3.0))
      (Class|DialogueComponent|AddLine _returnvalue_5 "F" 3.0))
    (:then_1
      (Class|DialogueComponent|AddLinetoBranch _returnvalue_4 (Utilities|Struct|MakeBranchInput 1 "G") 3.0)
      (Class|DialogueComponent|AddLine 0 "H" 3.0))))

(fn HideTemporary
  (bind _narratorwidget (Variables|Default|GetNarratorWidget))
  (bind _talkerwidget (Variables|Default|GetTalkerWidget))
  (if (Variables|Default|GetbNarrator)
    (Default|HideWidget _narratorwidget)
    (Default|ClearText _narratorwidget)
    (else
      (Class|BPITextBoxInterface|HideWidget(Message) _talkerwidget)
      (Class|BPITextBoxInterface|ClearText(Message) _talkerwidget))))

(fn GetActorLocationinViewport
  (params (TargetActor :type Actor%20Object%20Reference))
  (bind _returnvalue (Game|GetPlayerController 0))
  (bind _returnvalue_2 (Transformation|GetActorLocation TargetActor))
  (bind _textboxoffset (Variables|Default|GetTextBoxOffset))
  (bind _returnvalue_3 (+ _returnvalue_2 _textboxoffset))
  (bind (_screenposition _returnvalue_4) (Class|WidgetLayoutLibrary|ProjectWorldLocationtoWidgetPosition _returnvalue _returnvalue_3 false))
  (return _screenposition _returnvalue_4))

(fn UpdateWidgetPosition
  (bind _talkerwidget (Variables|Default|GetTalkerWidget))
  (if (not (Variables|Default|GetbNarrator))
    (if (Utilities|IsValid _talkerwidget)
      (bind (_viewport_position _actorinviewport_) (CallFunction|GetActorLocationinViewport (Components|GetOwner)))
      (Class|BPITextBoxInterface|SetPosition(Message) _talkerwidget _viewport_position))))

(fn UserRequestNext
  (if (Variables|Default|GetbSkippable)
    (Utilities|Time|ClearandInvalidateTimerbyHandle (Variables|Default|GetNextLineTimer))
    (Class|DialogueComponent|Next)))