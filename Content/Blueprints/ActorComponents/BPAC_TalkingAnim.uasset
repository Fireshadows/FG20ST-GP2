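; Actor component that fakes a talking animation by pulsing its owning actor's scale.
; Playanimation caches the owner's original scale and starts a looping timer that calls ScaleAnim.
; ScaleAnim uses a FlipFlop to alternate the owner between an offset scale and the original.
; Stopanimation clears the timer and restores the cached scale.
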(event Custom|ScaleAnim
  (bind _original_scale (Variables|Default|GetOriginal%20Scale))
  (Utilities|FlowControl|FlipFlop
    (:A
      (Variables|Default|SetTarget%20Scale (+ _original_scale (Variables|Default|GetScaleOffset))))
    (:B
      (Variables|Default|SetTarget%20Scale _original_scale)))
  (Transformation|SetActorScale3D (Components|GetOwner) (Variables|Default|GetTarget%20Scale)))

(event Custom|Play%20animation
  (bind _time (Variables|Default|GetTime))
  (Variables|Default|SetOriginal%20Scale (Transformation|GetActorScale3D (Components|GetOwner)))
  (bind _returnvalue (Utilities|Time|SetTimerbyEvent (delegate Custom|ScaleAnim) _time true (* _time 0.5)))
  (Variables|Default|SetTimerHandle _returnvalue))

(event Custom|Stop%20animation
  (Utilities|Time|ClearandInvalidateTimerbyHandle (Variables|Default|GetTimerHandle))
  (Transformation|SetActorScale3D (Components|GetOwner) (Variables|Default|GetOriginal%20Scale)))