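; BP_Viking is a puzzle character that reacts to the item the player brings to it and then completes the room.
; On overlap it allows one choice: a money pouch is destroyed and starts the Greed dialogue, while an actor with a BPAC_SwordTest component starts the Scared dialogue.
; When either dialogue finishes talking, it calls OnRoomFinished on BP_Gamestate.
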(event Custom|GreedResult
  (bind _asbp_gamestate (Utilities|Casting|CastToBP_Gamestate (Game|GetGameState)))
  (Default|OnRoomFinished _asbp_gamestate))

(event Custom|ScaredResult
  (bind _asbp_gamestate (Utilities|Casting|CastToBP_Gamestate (Game|GetGameState)))
  (Default|OnRoomFinished _asbp_gamestate))

(event EventBeginPlay
  (EventDispatchers|BindEventtoFinishedTalking (Variables|Default|GetGreed) (delegate Custom|GreedResult))
  (EventDispatchers|BindEventtoFinishedTalking (Variables|Default|GetScared) (delegate Custom|ScaredResult)))

(event Collision|EventActorBeginOverlap
  (params (OtherActor :type Actor%20Object%20Reference))
  (if (not (Variables|Default|GetChoiceMade))
    (if (== (Utilities|GetClass OtherActor) "/Game/Blueprints/VikingPuzzle/BP_MoneyPouch.BP_MoneyPouch_C")
      (Actor|DestroyActor OtherActor)
      (Class|SubtitleComponent|Start (Variables|Default|GetGreed))
      (Variables|Default|SetChoiceMade true :!label _label)
      (elif (Utilities|IsValid (Actor|GetComponentbyClass OtherActor "/Game/Blueprints/VikingPuzzle/BPAC_SwordTest.BPAC_SwordTest_C"))
        (Class|SubtitleComponent|Start (Variables|Default|GetScared))
        (goto _label)))))

(event EventTick
  (params (DeltaSeconds :type Float%20%28single-precision%29)))

(fn ConstructionScript)