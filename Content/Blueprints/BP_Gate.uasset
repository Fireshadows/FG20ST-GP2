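; BP_Gate is a locked gate that opens once its talker component has finished talking and every actor in its key list has overlapped it.
; Each matching key is destroyed and removed; the last starts a timeline that nudges the grid door along local Z and calls OnRoomFinished on BP_Gamestate every update.
; Separately, a stick hitbox snaps one targeted Snappable actor to StickSocket and disables its dragging.
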(event OnComponentBeginOverlap(StickhHitbox)
  (params (OverlappedComponent :type Primitive%20Component%20Object%20Reference) (OtherActor :type Actor%20Object%20Reference) (OtherComp :type Primitive%20Component%20Object%20Reference) (OtherBodyIndex :type Integer) (bFromSweep :type Boolean) (SweepResult :type Hit%20Result%20Structure%20%28by%20ref%29))
  (bind _returnvalue (Components|GetOwner OtherComp))
  (bind _returnvalue_2 (Actor|GetComponentbyClass _returnvalue "/Game/Blueprints/BPAC_Snappable.BPAC_Snappable_C"))
  (bind _returnvalue_3 (Actor|GetComponentbyClass _returnvalue "/Game/Blueprints/BPAC_Draggable.BPAC_Draggable_C"))
  (if (Utilities|IsValid OtherComp)
    (if (and (Utilities|IsValid _returnvalue_2) (== (Variables|/Game/Blueprints/BPAC_Snappable.BPAC_Snappable_C|GetTargetActor _returnvalue_2) self))
      (Utilities|IsValid (Variables|Default|GetSnapped%20Actor)
        (:Is%20Not%20Valid
          (Transformation|AttachActorToActor _returnvalue self "StickSocket" "SnapToTarget" "SnapToTarget" "SnapToTarget" true)
          (Variables|Default|SetSnapped%20Actor _returnvalue)
          (if (Utilities|IsValid _returnvalue_3)
            (Variables|/Script/FGGP2.InteractBaseComponent|Setinteractable _returnvalue_3 false)))))))

(event Collision|EventActorBeginOverlap
  (params (OtherActor :type Actor%20Object%20Reference))
  (if (and (Variables|/Game/Blueprints/BPAC_TalkerComponent.BPAC_TalkerComponent_C|GetFinishedTalking? (Variables|Default|GetBPAC_TalkerComponent)) (> (Utilities|Array|Length (Variables|Default|GetKeyList)) 0))
    (for _array_element (Variables|Default|GetKeyList)
      (if (== OtherActor _array_element)
        (Actor|DestroyActor _array_element)
        (Utilities|Array|RemoveItem (Variables|Default|GetKeyList) _array_element)
        (if (== (Utilities|Array|Length (Variables|Default|GetKeyList)) 0)
          (Timeline|Timeline_0 Play
            (:Update
              (Transformation|AddLocalOffset (Variables|Default|GetS_gridDoor) "0,0.000000,1.000000" false false)
              (bind _asbp_gamestate (Utilities|Casting|CastToBP_Gamestate (Game|GetGameState)))
              (Default|OnRoomFinished _asbp_gamestate))))))))

(fn ConstructionScript)