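; BP_Corpse is a Room3 corpse prop with a skeletal mesh that settles, freezes and can then be dragged.
; After a delay on BeginPlay, it puts rigid bodies to sleep by socket name and binds to the BPACDraggable component's Dragging event inside that loop.
; Each drag update sleeps the bodies again, then teleports the mesh to the new relative location without sweeping.
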(event Custom|Dragging
  (params (NewLocation :type Vector))
  (bind _skeletalmesh (Variables|Default|GetSkeletalMesh))
  (for _array_element (Transformation|GetAllSocketNames _skeletalmesh)
    (Class|PrimitiveComponent|PutRigidBodytoSleep _skeletalmesh _array_element))
  (Transformation|SetRelativeLocation _skeletalmesh NewLocation false true))

(event EventBeginPlay
  (bind _skeletalmesh (Variables|Default|GetSkeletalMesh))
  (Utilities|FlowControl|Delay (Variables|Default|GetTime%20until%20freeze))
  (for _array_element (Transformation|GetAllSocketNames _skeletalmesh)
    (Class|PrimitiveComponent|PutRigidBodytoSleep _skeletalmesh _array_element)
    (EventDispatchers|BindEventtoDragging (Variables|Default|GetBPAC_Draggable) (delegate Custom|Dragging))))

(event Collision|EventActorBeginOverlap
  (params (OtherActor :type Actor%20Object%20Reference)))

(event EventTick
  (params (DeltaSeconds :type Float%20%28single-precision%29)))

(fn ConstructionScript)