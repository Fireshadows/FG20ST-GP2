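; BP_EatingActor is a Room 3 puzzle actor that consumes a corpse or flute and completes the room.
; The first overlapping BP_Corpse or BP_Flute is destroyed, starts the Talk component and sets Satisfied so later overlaps are ignored.
; When talking finishes, a callback bound at BeginPlay calls OnRoomFinished on BP_Gamestate.
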(event Custom|Pass
  (bind _asbp_gamestate (Utilities|Casting|CastToBP_Gamestate (Game|GetGameState)))
  (Default|OnRoomFinished _asbp_gamestate))

(event EventBeginPlay
  (EventDispatchers|BindEventtoFinishedTalking (Variables|Default|GetTalk) (delegate Custom|Pass)))

(event Collision|EventActorBeginOverlap
  (params (OtherActor :type Actor%20Object%20Reference))
  (bind _returnvalue (Utilities|GetClass OtherActor))
  (if (and (not (Variables|Default|GetSatisfied)) (or (== _returnvalue "/Game/Blueprints/Room3/BP_Corpse.BP_Corpse_C") (== _returnvalue "/Game/Blueprints/Room2/BP_Flute.BP_Flute_C")))
    (Actor|DestroyActor OtherActor)
    (Class|SubtitleComponent|Start (Variables|Default|GetTalk))
    (Variables|Default|SetSatisfied true)))

(fn ConstructionScript)