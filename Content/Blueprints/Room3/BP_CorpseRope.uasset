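; BP_CorpseRope is a hanging corpse that can be cut down once by overlapping an actor with a BPAC_SwordTest component.
; The cut spawns a BP_Corpse and a scaled-up BP_MoneyPouch at the skeletal mesh's relative location, then hides the original mesh.
; The new corpse takes the same mesh, simulates physics, and briefly uses the original as master pose before being released, apparently to carry over the pose.
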(event Collision|EventActorBeginOverlap
  (params (OtherActor :type Actor%20Object%20Reference))
  (bind _skeletalmesh (Variables|Default|GetSkeletalMesh))
  (bind _skeletalmesh_2 (Variables|Default|GetSkeletalMesh))
  (bind _returnvalue (Transformation|GetRelativeTransform _skeletalmesh_2))
  (bind (_location _rotation) (Math|Transform|BreakTransform _returnvalue))
  (if (not (Variables|Default|GetHasBeenCut))
    (if (Utilities|IsValid (Actor|GetComponentbyClass OtherActor "/Game/Blueprints/Room3/BPAC_SwordTest.BPAC_SwordTest_C"))
      (bind _returnvalue_2 (Game|SpawnActorfromClass "/Game/Blueprints/Room3/BP_Corpse.BP_Corpse_C" (Math|Transform|MakeTransform _location _rotation (.Scale (Math|Transform|BreakTransform (Transformation|GetActorTransform)))) "Undefined" 0 0))
      (Game|SpawnActorfromClass "/Game/Blueprints/Room3/BP_MoneyPouch.BP_MoneyPouch_C" (Math|Transform|MakeTransform _location "0, 0, 0" "8.000000,8.000000,8.000000") "AlwaysSpawn" 0 0)
      (Variables|Default|SetHasBeenCut true)
      (Class|SkinnedMeshComponent|SetSkeletalMesh (Actor|GetComponentbyClass _returnvalue_2 "/Script/Engine.SkeletalMeshComponent") (Variables|/Script/Engine.SkinnedMeshComponent|GetSkeletalMesh _skeletalmesh) false)
      (Physics|SetSimulatePhysics (Actor|GetComponentbyClass _returnvalue_2 "/Script/Engine.SkeletalMeshComponent") true)
      (Class|SkinnedMeshComponent|SetMasterPoseComponent (Actor|GetComponentbyClass _returnvalue_2 "/Script/Engine.SkeletalMeshComponent") (Variables|Default|GetSkeletalMesh) false)
      (Class|SkinnedMeshComponent|SetMasterPoseComponent (Actor|GetComponentbyClass _returnvalue_2 "/Script/Engine.SkeletalMeshComponent") 0 false)
      (Rendering|SetVisibility _skeletalmesh false true))))

(event EventTick
  (params (DeltaSeconds :type Float%20%28single-precision%29)))

(fn ConstructionScript)