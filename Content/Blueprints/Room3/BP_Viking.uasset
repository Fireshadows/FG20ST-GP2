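; BP_Viking is Sven, the Room 3 ferryman NPC who outlines on hover and offers passage across the river.
; TextComponent runs his branching dialogue, which ReceiveItem resolves with a money pouch (good choice) or a sword.
; SinComponent separately answers offered sin objects, rewarding the matching one, and hides its text on a resettable timer.
; BP_Gamestate receives fate updates from both, plus room completion when the main dialogue stops.
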(event AnimatedTextLineFinished(TextComponent)
  (bind _textcomponent (Variables|Default|GetTextComponent))
  (Utilities|FlowControl|Delay (Variables|Default|GetDelayForNextLine))
  (Class|DialogueComponent|Next _textcomponent)
  (if (Class|DialogueComponent|AtBranch _textcomponent)
    (Default|HideTemporary (Variables|Default|GetTextComponent))))

(event DialogueStopped(TextComponent)
  (bind _gamestate (Variables|Default|GetGameState))
  (Default|OnRoomFinished _gamestate)
  (Default|UpdateFatePoint _gamestate (Variables|Default|GetbGoodChoice)))

(event DialogueStarted(SinComponent)
  (Utilities|Time|ClearandInvalidateTimerbyHandle (Variables|Default|GetTimerHandle))
  (bind _returnvalue (Utilities|Time|SetTimerbyEvent (delegate Custom|HideText) (Variables|Default|GetTimerUntilTextHide)))
  (Variables|Default|SetTimerHandle _returnvalue))

(event DialogueNext(SinComponent)
  (Utilities|Time|ClearandInvalidateTimerbyHandle (Variables|Default|GetTimerHandle))
  (bind _returnvalue (Utilities|Time|SetTimerbyEvent (delegate Custom|HideText) (Variables|Default|GetTimerUntilTextHide)))
  (Variables|Default|SetTimerHandle _returnvalue))

(event Custom|HideText
  (Default|HideTemporary (Variables|Default|GetSinComponent)))

(event EventBeginPlay
  (CallFunction|SetupText)
  (bind _asbp_gamestate (Utilities|Casting|CastToBP_Gamestate (Game|GetGameState)))
  (bind _output_get (Variables|Default|SetGameState _asbp_gamestate))
  (Variables|/Game/Blueprints/Core/BP_Gamestate.BP_Gamestate_C|SetViking _output_get self))

(event EventStartHovering
  (Rendering|SetRenderCustomDepth (Variables|Default|GetSkeletalMesh) true))

(event EventStopHovering
  (Rendering|SetRenderCustomDepth (Variables|Default|GetSkeletalMesh) false))

(fn ConstructionScript)

(fn SetupText
  (bind _sincomponent (Variables|Default|GetSinComponent))
  (bind _returnvalue (Class|DialogueComponent|InitializeText (Variables|Default|GetTextComponent) "Hail! I’ll take you over the river in exchange for coin." 0.0))
  (bind _returnvalue_2 (Class|DialogueComponent|AddLine (Variables|Default|GetTextComponent) _returnvalue "Charon? No, I’m Sven." 0.0))
  (bind _returnvalue_3 (Class|DialogueComponent|AddBranch (Variables|Default|GetTextComponent) _returnvalue_2))
  (Utilities|FlowControl|Sequence
    (:then_0
      (Class|DialogueComponent|AddLinetoBranch (Variables|Default|GetTextComponent) _returnvalue_3 (Utilities|Struct|MakeBranchInput (Variables|Default|GetSwordKey) "Augh! Watch where you point that thing. I get it, alright. I’ll take you over the river. No charge. Just don't hurt me!") 0.0))
    (:then_1
      (Class|DialogueComponent|AddLinetoBranch (Variables|Default|GetTextComponent) _returnvalue_3 (Utilities|Struct|MakeBranchInput (Variables|Default|GetMoneyKey) "Well, that amounts to about... Well, I don’t know what this one is worth, or that one, or that one, but this one! I’ll take that. Hop on board!") 0.0))
    (:then_2
      (bind _returnvalue_4 (Class|DialogueComponent|InitializeText (Variables|Default|GetSinComponent) "" 0.0))
      (Utilities|FlowControl|Sequence
        (:then_0
          (Class|DialogueComponent|AddLinetoBranch _sincomponent _returnvalue_4 (Utilities|Struct|MakeBranchInput (Variables|Default|GetSinKey) "Oh... I see. I guess you know, then. I won’t defend myself. Not here. Hel knows what I did, and I accept that now.") 2.0))
        (:then_1
          (Class|DialogueComponent|AddLinetoBranch _sincomponent _returnvalue_4 (Utilities|Struct|MakeBranchInput (Variables|Default|GetWrongSin) "Uh... Is this your diary or something? I don’t really need that.") 2.0))))))

(fn StartTalking
  (Class|DialogueComponent|Start (Variables|Default|GetTextComponent)))

(fn ReceiveItem
  (params (Actor :type Actor%20Object%20Reference) (Collider :type Actor%20Component%20Object%20Reference))
  (if (Variables|Default|GetChoiceMade)
    _
    (elif (== (Utilities|GetClass Actor) "/Game/Blueprints/Room3/BP_MoneyPouch.BP_MoneyPouch_C")
      (Actor|DestroyActor Actor)
      (Class|DialogueComponent|EnterKeyword (Variables|Default|GetTextComponent) (Variables|Default|GetMoneyKey))
      (Variables|Default|SetbGoodChoice true)
      (Variables|Default|SetChoiceMade true :!label _label)
      (return true)
      (elif (Utilities|IsValid (Actor|GetComponentbyClass Actor "/Game/Blueprints/Room3/BPAC_SwordTest.BPAC_SwordTest_C"))
        (Class|DialogueComponent|EnterKeyword (Variables|Default|GetTextComponent) (Variables|Default|GetSwordKey))
        (goto _label)
        (else
          _))))
  (bind _asbp_sin_object (Utilities|Casting|CastToBP_SinObject Actor)
    (:then
      (if (Utilities|Enum|Equal(Enum) (Variables|Default|GetSin) (Variables|/Game/Blueprints/BP_SinObject.BP_SinObject_C|GetAssociatedSin _asbp_sin_object))
        (Class|DialogueComponent|Start (Variables|Default|GetSinComponent))
        (Class|DialogueComponent|EnterKeyword (Variables|Default|GetSinComponent) (Variables|Default|GetSinKey))
        (Actor|DestroyActor Actor)
        (Default|UpdateFatePoint (Variables|Default|GetGameState) true)
        (return true)
        (else
          (Class|DialogueComponent|EnterKeyword (Variables|Default|GetSinComponent) (Variables|Default|GetWrongSin))
          (return false))))
    (:CastFailed
      (return false))))