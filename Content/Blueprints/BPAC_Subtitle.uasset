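; Subtitle component that displays timed or clickable dialogue lines through a widget implementing BPI_Subtitle.
; One second after BeginPlay it finds that widget and binds a switch on subtitle events: Started, Next and Finished.
; These show, update or hide the text, with Next also playing the line's sound and Finished flagging speech complete.
; Fixed-duration lines start a timer, while clicks pass only when Interactable.
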(event Custom|SubtitleEventSwitch
  (params (SubtitleEvent :type ESubtitleEvent%20Enum :default "SubtitleFinished"))
  (switch Utilities|FlowControl|Switch|SwitchonESubtitleEvent SubtitleEvent
    (:SubtitleFinished
      (CallFunction|StopShowingText)
      (Variables|Default|SetCompletedSpeech true))
    (:SubtitleStarted
      (CallFunction|StartShowingText))
    (:SubtitleNext
      (CallFunction|NewTexttoShow))))

(event EventClickable
  (|CanClick?)
  (Class|SubtitleComponent|Clicked))

(event EventBeginPlay
  (Utilities|FlowControl|Delay 1.0)
  (bind _foundwidgets (Class|WidgetBlueprintLibrary|GetAllWidgetswithInterface "/Game/Blueprints/BPI_Subtitle.BPI_Subtitle_C" false))
  (for _array_element _foundwidgets
    (Development|PrintString (Utilities|GetDisplayName _array_element))
    (Variables|Default|SetSubtitles (Utilities|Array|Get(acopy) _foundwidgets))
    (EventDispatchers|BindEventtoSubtitleEvent (delegate Custom|SubtitleEventSwitch))))

(fn StartShowingText
  (Class|BPISubtitle|ShowWidget(Message) (Variables|Default|GetSubtitles))
  (bind _returnvalue (Class|SubtitleComponent|GetCurrentTextData))
  (Class|BPISubtitle|SetText(Message) (Variables|Default|GetSubtitles) (.line (Utilities|Struct|BreakTextData _returnvalue)))
  (CallFunction|ManageText))

(fn StopShowingText
  (bind _subtitles (Variables|Default|GetSubtitles))
  (Class|BPISubtitle|HideWidget(Message) _subtitles)
  (Class|BPISubtitle|ClearText(Message) _subtitles))

(fn NewTexttoShow
  (bind _returnvalue (Class|SubtitleComponent|GetCurrentTextData))
  (Class|BPISubtitle|SetText(Message) (Variables|Default|GetSubtitles) (.line (Utilities|Struct|BreakTextData _returnvalue)))
  (Audio|PlaySoundatLocation (.soundRef (Utilities|Struct|BreakTextData _returnvalue)) "0, 0, 0" "0, 0, 0" 1.0 1.0 0.0 0 0 0)
  (CallFunction|ManageText))

(fn ManageText
  (bind _returnvalue (Class|SubtitleComponent|GetCurrentTextData))
  (switch Utilities|FlowControl|Switch|SwitchonENextLineTrigger (.triggerType (Utilities|Struct|BreakTextData _returnvalue))
    (:OnFixedDuration
      _)
    (:OnFixedDurationOrClick
      _))
  (Class|SubtitleComponent|StartTimer (.duration (Utilities|Struct|BreakTextData _returnvalue))))