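; Camera actor Blueprint that pans between two target points to move the view between segments.
; The MoveCamera event plays a timeline whose Pan track linearly interpolates the actor's location from TargetPoint1 to TargetPoint2.
; The MoveCameraGate function is empty apart from a disconnected copy of the move with a fixed zero alpha.
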(event Custom|MoveCamera
  ;[1 1 1] Camera pan between segments
  (bind _pan (Timeline|Timeline_0 Play)
    (:Update
      (Transformation|SetActorLocation (+ (Transformation|GetActorLocation (Variables|Default|GetTargetPoint1)) (* (- (Transformation|GetActorLocation (Variables|Default|GetTargetPoint2)) (Transformation|GetActorLocation (Variables|Default|GetTargetPoint1))) _pan)) false false))))

(fn ConstructionScript)

(fn MoveCameraGate
  ;[1 1 1] Camera pan between segments
)