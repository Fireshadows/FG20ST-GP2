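; Anubis judge for Room 4 that weighs the player's heart against a feather to decide the game's ending.
; On BeginPlay it spawns scales, heart and feather, and sets up both verdict lines.
; Judgement chains timelines that lower both items, attach them to the bowls, rock and level the scales, then tip them by comparing GameState FatePoints to GoodThreshold.
; The matching dialogue plays, and its end triggers BeginEnding on the GameState.
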(event DialogueStopped(DialogueComponent)
  (Development|PrintString "Dialogue Ended!" true true "(R=0.951570,G=1.000000,B=0.943905,A=1.000000)"))

(event Custom|Judgement
  (bind _scales (Variables|Default|GetScales))
  (bind _bowloscillationamount (Variables|Default|GetBowlOscillationAmount))
  (bind _heart (Variables|Default|GetHeart))
  (bind _lbowl (Variables|Default|GetLBowl))
  (bind _feather (Variables|Default|GetFeather))
  (bind _rbowl (Variables|Default|GetRBowl))
  (bind _bowloscillationamount_2 (Variables|Default|GetBowlOscillationAmount))
  (bind _returnvalue (Transformation|GetWorldLocation _rbowl))
  (bind _returnvalue_2 (Transformation|GetWorldLocation _lbowl))
  (bind (_x _y _z) (Math|Vector|BreakVector _returnvalue))
  (bind (_x_2 _y_2 _z_2) (Math|Vector|BreakVector _returnvalue_2))
  (Class|DialogueComponent|Start (Variables|Default|GetDialogueComponent))
  (bind _asbp_gamestate (Utilities|Casting|CastToBP_Gamestate (Game|GetGameState)))
  (Variables|Default|SetFatePoints (Variables|/Game/Blueprints/Core/BP_Gamestate.BP_Gamestate_C|GetFatePoints _asbp_gamestate))
  ;[1 1 1] Apple + Feather descent
  (Variables|Default|SetHeartTargetLocation (Math|Vector|MakeVector _x_2 _y_2 (- _z_2 4e+01)))
  (Variables|Default|SetFeatherTargetLocation (Math|Vector|MakeVector _x _y (- _z 5e+01)))
  (bind _newtrack_0 (Timeline|TL_Descent PlayFromStart)
    (:Update
      (Transformation|SetActorRelativeLocation _heart (Math|Vector|Lerp(Vector) (Transformation|GetActorLocation _heart) (Variables|Default|GetHeartTargetLocation) _newtrack_0))
      (Transformation|SetActorRelativeLocation _feather (Math|Vector|Lerp(Vector) (Transformation|GetActorLocation _feather) (Variables|Default|GetFeatherTargetLocation) _newtrack_0)))
    (:Finished
      ;[1 1 1] Sets target position and makes Heart and Feather a child of their respective bowls (so they move with the bowl)
      (bind _output_get (Variables|Default|SetLBowlOrigPos (Variables|/Script/Engine.SceneComponent|GetRelativeLocation (Variables|Default|GetLBowl))))
      (Variables|Default|SetLBowlUp (Math|Vector|MakeVector (.X (Math|Vector|BreakVector _output_get)) (.Y (Math|Vector|BreakVector _output_get)) (+ (.Z (Math|Vector|BreakVector _output_get)) _bowloscillationamount_2)))
      (bind _output_get_2 (Variables|Default|SetLBowlDown (Math|Vector|MakeVector (.X (Math|Vector|BreakVector _output_get)) (.Y (Math|Vector|BreakVector _output_get)) (- (.Z (Math|Vector|BreakVector _output_get)) _bowloscillationamount_2))))
      (Variables|Default|SetLBowlTargetPos _output_get_2)
      (bind _output_get_3 (Variables|Default|SetRBowlOrigPos (Variables|/Script/Engine.SceneComponent|GetRelativeLocation (Variables|Default|GetRBowl))))
      (Variables|Default|SetRBowlDown (Math|Vector|MakeVector (.X (Math|Vector|BreakVector _output_get_3)) (.Y (Math|Vector|BreakVector _output_get_3)) (- (.Z (Math|Vector|BreakVector _output_get_3)) _bowloscillationamount)))
      (bind _output_get_4 (Variables|Default|SetRBowlUp (Math|Vector|MakeVector (.X (Math|Vector|BreakVector _output_get_3)) (.Y (Math|Vector|BreakVector _output_get_3)) (+ (.Z (Math|Vector|BreakVector _output_get_3)) _bowloscillationamount))))
      (Variables|Default|SetRBowlTargetPos _output_get_4)
      (Transformation|AttachComponentToComponent (Variables|Default|GetHeart) (Variables|/Game/Blueprints/Room4/BP_Scales.BP_Scales_C|GetBowlLeft _scales) "None" "KeepWorld" "KeepWorld" "KeepWorld" true)
      (Transformation|AttachComponentToComponent (Variables|Default|GetFeather) (Variables|/Game/Blueprints/Room4/BP_Scales.BP_Scales_C|GetBowlRight _scales) "None" "KeepWorld" "KeepWorld" "KeepWorld" true)
      ;[1 1 1] Oscillate up/down set nr of times
      (bind _newtrack_0_2 (Timeline|TL_Oscillate PlayFromStart)
        (:Update
          (CallFunction|OscillateBowls _newtrack_0_2))
        (:Finished
          (if (< (Variables|Default|GetTimesHaveOscillated) (Variables|Default|GetTimesToOscillateScales))
            (Variables|Default|SetTimesHaveOscillated (+ (Variables|Default|GetTimesHaveOscillated) 1))
            (CallFunction|FlipBowlTargetPos)
            (Timeline|TL_Oscillate PlayFromStart)
            (else
              (Variables|Default|SetLBowlTargetPos (Variables|Default|GetLBowlOrigPos))
              (Variables|Default|SetRBowlTargetPos (Variables|Default|GetRBowlOrigPos))
              (bind _newtrack_0_3 (Timeline|TL_ResetPosition PlayFromStart)
                (:Update
                  (CallFunction|ReturnBowltoOriginalPosition _newtrack_0_3))
                (:Finished
                  ;[1 1 1] Compare score + + final oscillation + narrate result
                  (if (< (Variables|Default|GetFatePoints) (Variables|Default|GetGoodThreshold))
                    (Variables|Default|SetGood%20Ending false)
                    (Variables|Default|SetLBowlTargetPos (Variables|Default|GetLBowlDown)) ; Bad ending; heavy heart
                    (Variables|Default|SetRBowlTargetPos (Variables|Default|GetRBowlUp))
                    (Variables|Default|SetTargetCrossbarRotation "0, 0,15.000000")
                    (Class|DialogueComponent|EnterKeyword (Variables|Default|GetDialogueComponent) (Variables|Default|GetBadEnding))
                    (bind _newtrack_0_4 (Timeline|TL_FinalMovement PlayFromStart)
                      (:Update
                        (CallFunction|OscillateBowls _newtrack_0_4)))
                    (else
                      (Variables|Default|SetGood%20Ending true)
                      (Variables|Default|SetLBowlTargetPos (Variables|Default|GetLBowlUp)) ; Good ending; light heart
                      (Variables|Default|SetRBowlTargetPos (Variables|Default|GetRBowlDown))
                      (Variables|Default|SetTargetCrossbarRotation "0, 0,-15.000000")
                      (Class|DialogueComponent|EnterKeyword (Variables|Default|GetDialogueComponent) (Variables|Default|GetGoodEnding))
                      (Timeline|TL_FinalMovement PlayFromStart))))))))))))

(event Custom|OnFinishedTalking
  (bind _asbp_gamestate (Utilities|Casting|CastToBP_Gamestate (Game|GetGameState)))
  (Default|BeginEnding _asbp_gamestate (Variables|Default|GetGood%20Ending)))

(event EventBeginPlay
  (bind _returnvalue (Transformation|GetActorTransform))
  (bind _location (Math|Transform|BreakTransform _returnvalue))
  (bind (_x _y _z) (Math|Vector|BreakVector _location))
  (bind _returnvalue_2 (Game|SpawnActorfromClass "/Game/Blueprints/Room4/BP_Scales.BP_Scales_C" (Math|Transform|MakeTransform (Math|Vector|MakeVector (- _x 1e+02) _y (- _z 1e+02)) "0,180.000000, 0" "3.000000,3.000000,3.000000") "Undefined" 0 0))
  (bind _output_get (Variables|Default|SetScales _returnvalue_2))
  (bind _output_get_2 (Variables|Default|SetLBowl (Variables|/Game/Blueprints/Room4/BP_Scales.BP_Scales_C|GetBowlLeft _output_get)))
  (Variables|Default|SetRBowl (Variables|/Game/Blueprints/Room4/BP_Scales.BP_Scales_C|GetBowlRight _output_get))
  (Variables|Default|SetCrossbar (Variables|/Game/Blueprints/Room4/BP_Scales.BP_Scales_C|GetCrossbar _output_get))
  (bind _returnvalue_3 (Game|SpawnActorfromClass "/Game/Blueprints/Room4/BP_Heart.BP_Heart_C" (Math|Transform|MakeTransform (Math|Vector|MakeVector (.X (Math|Vector|BreakVector (.Location (Math|Transform|BreakTransform (Transformation|GetWorldTransform _output_get_2))))) (.Y (Math|Vector|BreakVector (.Location (Math|Transform|BreakTransform (Transformation|GetWorldTransform _output_get_2))))) (+ (.Z (Math|Vector|BreakVector (.Location (Math|Transform|BreakTransform (Transformation|GetWorldTransform _output_get_2))))) 5e+02)) "0.000000,180.000000,0.000000") "Undefined" 0 0))
  (Variables|Default|SetHeart _returnvalue_3)
  (bind _returnvalue_4 (Game|SpawnActorfromClass "/Game/Blueprints/Room4/BP_Feather.BP_Feather_C" (Math|Transform|MakeTransform (Math|Vector|MakeVector (.X (Math|Vector|BreakVector (.Location (Math|Transform|BreakTransform (Transformation|GetWorldTransform (Variables|Default|GetRBowl)))))) (.Y (Math|Vector|BreakVector (.Location (Math|Transform|BreakTransform (Transformation|GetWorldTransform (Variables|Default|GetRBowl)))))) (+ (.Z (Math|Vector|BreakVector (.Location (Math|Transform|BreakTransform (Transformation|GetWorldTransform (Variables|Default|GetRBowl)))))) 5e+02)) "0,180.000000, 0") "Undefined" 0 0))
  (Variables|Default|SetFeather _returnvalue_4)
  (CallFunction|SetupText)
  (EventDispatchers|BindEventtoDialogueStopped (Variables|Default|GetDialogueComponent) (delegate Custom|OnFinishedTalking)))

(fn ConstructionScript)

(fn FlipBowlTargetPos
  (if (== (Math|Integer|%(Integer) (Variables|Default|GetTimesHaveOscillated) 2) 0)
    (Variables|Default|SetLBowlTargetPos (Variables|Default|GetLBowlDown))
    (Variables|Default|SetRBowlTargetPos (Variables|Default|GetRBowlUp))
    (Variables|Default|SetTargetCrossbarRotation "0, 0,15.000000")
    (else
      (Variables|Default|SetLBowlTargetPos (Variables|Default|GetLBowlUp))
      (Variables|Default|SetRBowlTargetPos (Variables|Default|GetRBowlDown))
      (Variables|Default|SetTargetCrossbarRotation "0, 0,-15.000000"))))

(fn OscillateBowls
  (params (delta :type Float%20%28single-precision%29))
  (bind _crossbar (Variables|Default|GetCrossbar))
  (bind _rbowl (Variables|Default|GetRBowl))
  (bind _lbowl (Variables|Default|GetLBowl))
  (Transformation|SetRelativeLocation _lbowl (Math|Vector|Lerp(Vector) (Variables|/Script/Engine.SceneComponent|GetRelativeLocation _lbowl) (Variables|Default|GetLBowlTargetPos) delta) false false)
  (Transformation|SetRelativeLocation _rbowl (Math|Vector|Lerp(Vector) (Variables|/Script/Engine.SceneComponent|GetRelativeLocation _rbowl) (Variables|Default|GetRBowlTargetPos) delta) false false)
  (Transformation|SetRelativeRotation _crossbar (Math|Rotator|Lerp(Rotator) (Variables|/Script/Engine.SceneComponent|GetRelativeRotation _crossbar) (Variables|Default|GetTargetCrossbarRotation) delta) false false))

(fn ReturnBowltoOriginalPosition
  (params (Delta :type Float%20%28single-precision%29))
  (bind _crossbar (Variables|Default|GetCrossbar))
  (bind _rbowl (Variables|Default|GetRBowl))
  (bind _lbowl (Variables|Default|GetLBowl))
  (Transformation|SetRelativeLocation _lbowl (Math|Vector|Lerp(Vector) (Variables|/Script/Engine.SceneComponent|GetRelativeLocation _lbowl) (Variables|Default|GetLBowlTargetPos) Delta) false false)
  (Transformation|SetRelativeLocation _rbowl (Math|Vector|Lerp(Vector) (Variables|/Script/Engine.SceneComponent|GetRelativeLocation _rbowl) (Variables|Default|GetRBowlTargetPos) Delta) false false)
  (Transformation|SetRelativeRotation _crossbar (Math|Rotator|Lerp(Rotator) (Variables|/Script/Engine.SceneComponent|GetRelativeRotation _crossbar) (Variables|Default|GetOriginalCrossbarRotation) Delta) false false))

(fn SetupText
  (bind _returnvalue (Class|DialogueComponent|InitializeText (Variables|Default|GetDialogueComponent) "" 0.0))
  (bind _returnvalue_2 (Class|DialogueComponent|AddBranch (Variables|Default|GetDialogueComponent) _returnvalue))
  (Utilities|FlowControl|Sequence
    (:then_0
      (Class|DialogueComponent|AddLinetoBranch (Variables|Default|GetDialogueComponent) _returnvalue_2 (Utilities|Struct|MakeBranchInput (Variables|Default|GetGoodEnding) "Now, what’s this? You seem to be in the wrong place. I wonder which of those  fools misplaced you here. Very well. You are granted your paradise.") 0.0))
    (:then_1
      (Class|DialogueComponent|AddLinetoBranch (Variables|Default|GetDialogueComponent) _returnvalue_2 (Utilities|Struct|MakeBranchInput (Variables|Default|GetBadEnding) "Well, well. You desire freedom, but continue to weigh heavy on my scales. Nothing has changed since you were placed here. No matter. Perhaps you will change in due time. Go back to your hole.") 0.0))))