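; Actor component that lets the player drag its owning actor with the mouse, keeping X fixed and optionally locking vertical or horizontal movement.
; Each Draggable call projects the cursor ray to the actor's current distance from it, moves the owner there and broadcasts Dragging.
; Interactable or uninteractable drag events fire once per press, re-armed on Tick when BP_Character's MouseClicked clears.
; StartDragging and StopDragging relay to their own dispatchers.
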(event EventStartDragging
  (Default|CallStartedDragging))

(event EventStopDragging
  (Default|CallStoppedDragging))

(event EventTick
  (params (DeltaSeconds :type Float%20%28single-precision%29))
  (Utilities|FlowControl|Sequence
    (:then_0
      (if (Variables|Default|GetInteractableEventClosed)
        (if (not (Variables|/Game/Blueprints/Core/BP_Character.BP_Character_C|GetMouseClicked (Variables|Default|GetCharacter)))
          (Variables|Default|SetInteractableEventClosed false)
          (Utilities|FlowControl|DoOnce false) ; enters at Reset
        )))
    (:then_1
      (if (Variables|Default|GetUninteractableEventClosed)
        (if (not (Variables|/Game/Blueprints/Core/BP_Character.BP_Character_C|GetMouseClicked (Variables|Default|GetCharacter)))
          (Variables|Default|SetUninteractableEventClosed false)
          (Utilities|FlowControl|DoOnce false) ; enters at Reset
        )))))

(event EventDraggable
  (if (Variables|Default|Getinteractable)
    (Utilities|FlowControl|Sequence
      (:then_0
        (bind _newparam (CallFunction|GetNewPosition))
        (Transformation|SetActorLocation (Components|GetOwner) _newparam false false)
        (Default|CallDragging _newparam))
      (:then_1
        (Utilities|FlowControl|DoOnce false
          (:Completed
            (Default|CallOnDragInteractable)
            (Variables|Default|SetInteractableEventClosed true)))))
    (else
      (Utilities|FlowControl|DoOnce false
        (:Completed
          (Default|CallOnDragUninteractable)
          (Variables|Default|SetUninteractableEventClosed true))))))

(event EventBeginPlay
  (bind _asbp_character (Utilities|Casting|CastToBP_Character (Game|Player|GetPlayerPawn 0)))
  (Variables|Default|SetCharacter _asbp_character))

(fn GetNewPosition
  (bind _returnvalue (Game|GetPlayerController 0))
  (bind _returnvalue_2 (Components|GetOwner))
  (bind _returnvalue_3 (Components|GetOwner))
  (bind (_worldlocation _worlddirection) (Game|Player|ConvertMouseLocationToWorldSpace _returnvalue))
  (bind _returnvalue_4 (Transformation|GetActorLocation _returnvalue_2))
  (bind _returnvalue_5 (Transformation|GetActorLocation _returnvalue_3))
  (bind _returnvalue_6 (Math|Vector|Distance(Vector) _returnvalue_4 _worldlocation))
  (bind _returnvalue_7 (Math|Vector|Normalize _worlddirection))
  (bind (_x _y _z) (Math|Vector|BreakVector _returnvalue_5))
  (bind _returnvalue_8 (* _returnvalue_7 _returnvalue_6))
  (bind _returnvalue_9 (+ _worldlocation _returnvalue_8))
  (bind (_x_2 _y_2 _z_2) (Math|Vector|BreakVector _returnvalue_9))
  (LocalVariables|Setresult (Math|Vector|MakeVector (.X (Math|Vector|BreakVector _returnvalue_4)) _y_2 _z_2))
  (if (Variables|Default|GetLock%20Vertical)
    (LocalVariables|Setresult (Math|Vector|MakeVector (.X (Math|Vector|BreakVector (LocalVariables|Getresult))) (.Y (Math|Vector|BreakVector (LocalVariables|Getresult))) _z)))
  (if (Variables|Default|GetLock%20Horizontal)
    (LocalVariables|Setresult (Math|Vector|MakeVector (.X (Math|Vector|BreakVector (LocalVariables|Getresult))) _y (.Z (Math|Vector|BreakVector (LocalVariables|Getresult))))))
  (return (LocalVariables|Getresult)))