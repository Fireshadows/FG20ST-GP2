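; Player Blueprint for mouse-driven clicking and dragging of actors that carry an AC_Interactable component, with a visible cursor.
; Pressing Mouse1 caches the hit actor's component, and releasing it sends a click message to whatever component is then hit.
; While held, Tick passes the hit location to the cached component, which is never cleared.
; HitDetection supplies the hits, though its under-cursor visibility trace appears unconnected.
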(event EventBeginPlay
  (Variables|/Script/Engine.PlayerController|SetbShowMouseCursor (Game|GetPlayerController 0) true))

(event EventTick
  (params (DeltaSeconds :type Float%20%28single-precision%29))
  (bind _draggingcomponent (Variables|Default|GetDraggingComponent))
  (if (Variables|Default|GetMouseClicked)
    (if (Utilities|IsValid _draggingcomponent)
      (Class|BPInterfaces|Draggable(Message) _draggingcomponent (.Location (Collision|BreakHitResult (Utilities|HitDetection)))))))

(event Input|ActionEvents|InputActionMouse1
  (params (Key :type Key%20Structure :default "None"))
  (:Pressed
    (Variables|Default|SetMouseClicked true)
    (CallFunction|GetDragComponent))
  (:Released
    (CallFunction|GetClickComponent)
    (Variables|Default|SetMouseClicked false)))

(fn ConstructionScript)

(fn GetClickComponent
  (bind _result (Utilities|HitDetection))
  (bind _hitactor (Collision|BreakHitResult _result))
  (bind _returnvalue (Actor|GetComponentbyClass _hitactor "/Game/Blueprints/AC_Interactable.AC_Interactable_C"))
  (if (Utilities|IsValid _returnvalue)
    (Class|BPInterfaces|Clickable(Message) _returnvalue)))

(fn GetDragComponent
  (bind _result (Utilities|HitDetection))
  (bind _hitactor (Collision|BreakHitResult _result))
  (bind _returnvalue (Actor|GetComponentbyClass _hitactor "/Game/Blueprints/AC_Interactable.AC_Interactable_C"))
  (Utilities|IsValid _returnvalue
    (:Is%20Valid
      (Variables|Default|SetDraggingComponent _returnvalue))))