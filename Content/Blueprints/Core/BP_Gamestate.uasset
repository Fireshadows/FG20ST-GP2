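; Game state Blueprint that manages room-to-room progression, the main camera, HUD and a fate point score.
; BeginPlay caches the character, camera and parallax actors, creates HUD, inventory and arrow widgets, then enters the current room.
; Transitions and camera sequences disable character input, then restore it after per-room delays, refreshing arrows and camera offsets; room 3 starts Viking dialogue.
; Fate points resolve into one of three fates against a symmetric threshold.
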(event Custom|OnRoomEntered
  (params (Delay :type Float%20%28single-precision%29))
  (bind _currentroom (Variables|Default|GetCurrentRoom))
  (Utilities|FlowControl|Delay Delay)
  (Default|SetInput (Variables|Default|GetCharacter) true)
  (Default|ShowExtraHUD (Variables|Default|GetArrowHUD) _currentroom)
  (Default|UpdateCameraOffsetPositions (Variables|Default|GetMainCamera))
  (switch int _currentroom
    (:3
      (Default|StartTalking (Variables|Default|GetViking)))))

(event EventBeginPlay
  (bind _asbp_character (Utilities|Casting|CastToBP_Character (Game|GetPlayerCharacter 0)))
  (Variables|Default|SetCharacter _asbp_character)
  (bind _outactors (Actor|GetAllActorsOfClass "/Game/Blueprints/BP_Camera.BP_Camera_C"))
  (bind _camera (Class|BPICamera|GetCamera(Message) (Utilities|Array|Get(acopy) _outactors)))
  (Variables|Default|SetMainCamera _camera)
  (bind _outactors_2 (Actor|GetAllActorswithInterface "/Game/Blueprints/Interfaces/BPI_Parallax.BPI_Parallax_C"))
  (Variables|Default|SetParallaxArray _outactors_2)
  (bind _target_point (CallFunction|GetCurrentPoint))
  (Default|SnaptoTarget (Variables|Default|GetMainCamera) _target_point)
  ;[1 1 1] Create Widget
  (bind _returnvalue (UserInterface|CreateWidget "/Game/Blueprints/UI/WBP_MainHUD.WBP_MainHUD_C"))
  (UserInterface|Viewport|AddtoViewport _returnvalue 0)
  (bind _returnvalue_2 (UserInterface|CreateWidget "/Game/Blueprints/UI/Inventory/WBP_Inventory.WBP_Inventory_C" (Game|GetPlayerController 0)))
  (UserInterface|Viewport|AddtoViewport _returnvalue_2 0)
  (bind _returnvalue_3 (UserInterface|CreateWidget "/Game/Blueprints/UI/WBP_CameraMovementIndicator.WBP_CameraMovementIndicator_C"))
  (bind _output_get (Variables|Default|SetArrowHUD _returnvalue_3))
  (UserInterface|Viewport|AddtoViewport _output_get 0)
  (CallFunction|OnRoomEntered 0.0))

(fn ConstructionScript)

(fn OnRoomFinished
  (Default|ShowHUD (Variables|Default|GetArrowHUD)))

(fn RoomTransition
  (params (Transition%20to :type Target%20Point%20Object%20Reference))
  (bind _currentroom (Variables|Default|GetCurrentRoom))
  (bind _returnvalue (Utilities|Select :Index _currentroom :Option%200 3.0 :Option%201 3.0 :Option%202 3.0 :Option%203 0.0))
  (bind _target_point (CallFunction|GetCurrentPoint))
  (Default|MoveCamera (Variables|Default|GetMainCamera) _target_point Transition%20to _returnvalue)
  (Default|SetInput (Variables|Default|GetCharacter) false)
  (CallFunction|OnRoomEntered _returnvalue))

(fn GetIndex
  (if (< (Variables|Default|GetCurrentRoom) 0)
    (LocalVariables|SetIndex 0)
    (else
      (LocalVariables|SetIndex (Variables|Default|GetCurrentRoom))))
  (return (LocalVariables|GetIndex)))

(fn GetCurrentPoint
  (bind _maincamera (Variables|Default|GetMainCamera))
  (bind _targetpoints (Variables|/Game/Blueprints/BP_Camera.BP_Camera_C|GetTargetPoints _maincamera))
  (if (< (Variables|Default|GetCurrentRoom) (Utilities|Array|Length _targetpoints))
    (LocalVariables|SetCurrent%20Point (Utilities|Array|Get(acopy) _targetpoints (Variables|Default|GetCurrentRoom)))
    (else
      (Development|PrintString "Unavailable Room - Getting first room" true true "(R=1.000000,G=0.177017,B=0.186965,A=1.000000)")
      (LocalVariables|SetCurrent%20Point (Utilities|Array|Get(acopy) _targetpoints))))
  (return (LocalVariables|GetCurrent%20Point)))

(fn GetRoom
  (params (Index :type Integer))
  (return (Utilities|Array|Get(acopy) (Variables|/Game/Blueprints/BP_Camera.BP_Camera_C|GetTargetPoints (Variables|Default|GetMainCamera)) Index)))

(fn UpdateRoom
  (params (New%20Room%20Index :type Integer))
  (Variables|Default|SetCurrentRoom New%20Room%20Index))

(fn UpdateFatePoint
  (params (GainFatePoint :type Boolean))
  (if GainFatePoint
    (Variables|Default|SetFatePoints (+ (Variables|Default|GetFatePoints) 1))
    (else
      (Variables|Default|SetFatePoints (- (Variables|Default|GetFatePoints) 1))))
  (Development|PrintString (Utilities|String|ToString(Integer) (Variables|Default|GetFatePoints))))

(fn DetermineFate
  (if (<= (Variables|Default|GetFatePoints) (* (Variables|Default|GetFate%20Treshold) -1))
    (Variables|Default|SetFate "NewEnumerator2")
    (elif (< (Variables|Default|GetFatePoints) (Variables|Default|GetFate%20Treshold))
      (Variables|Default|SetFate "NewEnumerator0")
      (else
        (Variables|Default|SetFate "NewEnumerator1"))))
  (Development|PrintString (Utilities|String|EnumtoString (Variables|Default|GetFate))))

(fn GetXPositionforScreen
  (bind _draggingoffsets (Variables|Default|GetDraggingOffsets))
  (bind _newparam (CallFunction|GetIndex))
  (if (< _newparam (Utilities|Array|Length _draggingoffsets))
    (return (Utilities|Array|Get(acopy) _draggingoffsets _newparam))
    (else
      (return 0.0))))

(fn StartCamSequence
  (params (Sequence%20Index :type Integer))
  (Default|SequenceCamera (Variables|Default|GetMainCamera) Sequence%20Index)
  (Default|SetInput (Variables|Default|GetCharacter) false)
  (CallFunction|OnRoomEntered (Utilities|Select :Index (Variables|Default|GetCurrentRoom) :Option%200 5.0 :Option%201 3.0 :Option%202 0.0 :Option%203 5.53)))

(fn GetCamera
  (return (Variables|Default|GetMainCamera)))