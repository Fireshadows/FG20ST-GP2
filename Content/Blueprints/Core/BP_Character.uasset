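; Player character for a point-and-click game, handling cursor-driven camera panning, clicking, dragging, inventory and a pair-matching memory puzzle.
; Tick pans the view target within horizontal limits, notifies parallax actors, updates drags and refreshes cursor and hover-emissive feedback.
; Cursor hit tests route clicks to interact components, draggables or memory tiles, with delays before mismatches hide.
; Each matched pair moves BP_Greek, and the Zoom axis shifts dragged objects in depth.
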(event Custom|Set%20Input
  (params (enable :type Boolean))
  (if enable
    (Input|EnableInput 0)
    (Default|SetInventoryEnabled (Variables|Default|GetInventoryWidget) true)
    (else
      (Input|DisableInput 0)
      (Default|SetInventoryEnabled (Variables|Default|GetInventoryWidget) false))))

(event EventInventory
  (params (New%20Item :type Actor%20Object%20Reference))
  (bind _inventorycomponent (Variables|Default|GetInventoryComponent))
  ;[1 1 1] Inventory
  (bind _returnvalue (Class|Inventory|AddItem _inventorycomponent New%20Item))
  (if _returnvalue
    (Development|PrintString "Added")
    (Default|CallOnElementAdded (Utilities|Array|FindItem (Variables|/Script/FGGP2.Inventory|GetInventory _inventorycomponent) New%20Item) New%20Item)))

(event EventBeginPlay
  (bind _returnvalue (Game|GetPlayerController 0))
  (bind _returnvalue_2 (Viewport|GetViewportSize))
  (bind _returnvalue_3 (* _returnvalue_2 0.5))
  (bind (_x _y) (Math|Vector2D|BreakVector2D _returnvalue_3))
  ;[1 1 1] BeginPlay
  (Variables|/Script/Engine.PlayerController|SetbShowMouseCursor _returnvalue true)
  (bind _foundwidgets (Widget|GetAllWidgetsOfClass "/Game/Blueprints/UI/Inventory/WBP_Inventory.WBP_Inventory_C" true))
  (Utilities|IsValid (Utilities|Array|Get(acopy) _foundwidgets)
    (:Is%20Valid
      (Variables|Default|SetInventoryWidget (Utilities|Array|Get(acopy) _foundwidgets)))
    (:Is%20Not%20Valid
      _))
  (Class|PlayerController|SetMouseLocation _returnvalue (Math|Float|Truncate _x) (Math|Float|Truncate _y))
  (bind _returnvalue_4 (Actor|GetActorOfClass "/Game/Blueprints/BP_Camera.BP_Camera_C"))
  (bind _output_get (Variables|Default|SetCameraPosition (Transformation|GetActorLocation _returnvalue_4)))
  (Variables|Default|SetCameraPositionMaxLeft (Math|Vector|MakeVector (.X (Math|Vector|BreakVector _output_get)) (- (.Y (Math|Vector|BreakVector _output_get)) (Variables|Default|GetMaximumCameraHorizontalOffset)) (.Z (Math|Vector|BreakVector _output_get))))
  (Variables|Default|SetCameraPositionMaxRight (Math|Vector|MakeVector (.X (Math|Vector|BreakVector (Variables|Default|GetCameraPosition))) (+ (.Y (Math|Vector|BreakVector (Variables|Default|GetCameraPosition))) (Variables|Default|GetMaximumCameraHorizontalOffset)) (.Z (Math|Vector|BreakVector (Variables|Default|GetCameraPosition)))))
  (bind _asbp_gamestate (Utilities|Casting|CastToBP_Gamestate (Game|GetGameState)))
  (Variables|Default|SetGameState _asbp_gamestate)
  (bind _asgm_point_and_click (Utilities|Casting|CastToGM_PointAndClick (Game|GetGameMode)))
  (Variables|Default|SetGameMode _asgm_point_and_click)
  (bind _returnvalue_5 (Actor|GetActorOfClass "/Game/Blueprints/Characters/BP_Greek.BP_Greek_C"))
  (Variables|Default|SetSinGreek _returnvalue_5))

(event EventTick
  (params (DeltaSeconds :type Float%20%28single-precision%29))
  (bind _returnvalue (Viewport|GetViewportSize))
  (bind _returnvalue_2 (Game|GetPlayerController 0))
  (bind _returnvalue_3 (Game|GetPlayerCameraManager 0))
  (bind _returnvalue_4 (Game|GetPlayerController 0))
  (bind _draggingcomponent (Variables|Default|GetDraggingComponent))
  (bind _gamestate (Variables|Default|GetGameState))
  (bind (_deltax _deltay) (Class|PlayerController|GetInputMouseDelta _returnvalue_2))
  (bind _returnvalue_5 (Camera|GetCameraLocation _returnvalue_3))
  (bind _returnvalue_6 (* _returnvalue 0.5))
  (bind _returnvalue_7 (Pawn|GetViewTarget _returnvalue_4))
  (bind _parallaxarray (Variables|/Game/Blueprints/Core/BP_Gamestate.BP_Gamestate_C|GetParallaxArray _gamestate))
  (bind _x (Math|Vector2D|BreakVector2D _returnvalue_6))
  (bind _y (Math|Vector|BreakVector _returnvalue_5))
  ;[1 1 1] Event Tick - Camera Panning with cursor
  (Utilities|FlowControl|Sequence
    (:then_0
      (bind _returnvalue_8 (Class|WidgetLayoutLibrary|GetMousePositiononViewport))
      (bind _output_get (Variables|Default|SetMousePositionHorizontal (.X (Math|Vector2D|BreakVector2D (* _returnvalue_8 (Class|WidgetLayoutLibrary|GetViewportScale))))))
      (if (not (Math|Float|NearlyEqual(Float) _output_get _x (Variables|Default|GetCameraMovementLeniency)))
        (Math|Float|CompareFloat _output_get _x
          (:>
            (if (> (.Y (Math|Vector|BreakVector (Variables|Default|GetCameraPositionMaxRight))) _y) ; Player isn't too far right
              (Transformation|AddActorWorldOffset _returnvalue_7 "0.000000,5.000000,0.000000")
              ;[1 1 1] Parallax movement for anything with parallax interface
              (for _array_element _parallaxarray
                (Class|BPIParallax|ParallaxMovement(Message) _array_element false))))
          (:<
            (if (> _y (.Y (Math|Vector|BreakVector (Variables|Default|GetCameraPositionMaxLeft)))) ; Player isn't too far left
              (Transformation|AddActorWorldOffset _returnvalue_7 "0.000000,-5.000000, 0")
              (for _array_element_2 _parallaxarray
                (Class|BPIParallax|ParallaxMovement(Message) _array_element_2 true)))))))
    (:then_1
      ;;[1 1 1] Event Tick - Dragging
      (if (Variables|Default|GetMouseClicked)
        (if (Utilities|IsValid _draggingcomponent)
          (if (Variables|Default|GetIsDragging?)
            (Class|InteractInterface|Draggable(Message) _draggingcomponent)
            (elif (> (+ (Math|Float|Absolute(Float) _deltax) (Math|Float|Absolute(Float) _deltay)) 0.1)
              (Variables|Default|SetIsDragging? true)
              (Class|BPIDraggableInterface|StartDragging(Message) _draggingcomponent))))))
    (:then_2
      ;;[1 1 1] Hovering Detection
      (CallFunction|CursorLogic)
      (CallFunction|HoverableEmissive))))

(event Input|ActionEvents|InputActionMouse2
  (params (Key :type Key%20Structure :default "None"))
  ;[1 1 1] Mouse2
  (:Released
    ;[1 1 1] Mouse1
    (Utilities|IsValid (Variables|Default|GetDraggingComponent)
      (:Is%20Valid
        (Class|BPIDraggableInterface|StopDragging(Message) (Variables|Default|GetDraggingComponent))
        (Variables|Default|SetDraggingComponent 0))
      (:Is%20Not%20Valid
        _))
    (Variables|Default|SetMouseClicked false)
    (Variables|Default|SetIsDragging? false)))

(event Input|ActionEvents|InputActionMouse1
  (params (Key :type Key%20Structure :default "None"))
  ;[1 1 1] Mouse1
  (:Pressed
    (Variables|Default|SetMouseClicked true)
    (CallFunction|GetDragComponent)
    (if (Variables|Default|GetAcceptMemoryObjectInput)
      (bind _hideobjects (CallFunction|GetMemoryObject))
      (Utilities|FlowControl|Delay (Variables|Default|GetMemoryPuzzleObjectDelay))
      (CallFunction|HideMemoryObjects _hideobjects)
      (if (not _hideobjects)
        _
        (else
          (Utilities|FlowControl|Delay (/ (Variables|Default|GetMemoryPuzzleObjectDelay) 2.0)) ; To allow tiles to hide again.
        ))
      (Variables|Default|SetAcceptMemoryObjectInput true)
      (if (Variables|Default|GetCompletedAMemoryPuzzle)
        (Default|MovePosition (Variables|Default|GetSinGreek) (Variables|Default|GetMemoryPuzzlesCompleted))
        (Variables|Default|SetCompletedAMemoryPuzzle false))))
  (:Released
    (if (Variables|Default|GetIsDragging?)
      (Utilities|IsValid (Variables|Default|GetDraggingComponent)
        (:Is%20Valid
          (Class|BPIDraggableInterface|StopDragging(Message) (Variables|Default|GetDraggingComponent))
          (Variables|Default|SetDraggingComponent 0 :!label _label))
        (:Is%20Not%20Valid
          _))
      (else
        (CallFunction|GetClickComponent)
        (goto _label)))
    (Variables|Default|SetMouseClicked false)
    (Variables|Default|SetIsDragging? false)))

(event Input|ActionEvents|InputActionExit
  (params (Key :type Key%20Structure :default "None"))
  (:Pressed
    (Game|QuitGame 0 "Quit" false)))

(event Input|AxisEvents|InputAxisZoom
  (params (AxisValue :type Float%20%28single-precision%29))
  (bind _draggingcomponent (Variables|Default|GetDraggingComponent))
  (bind _returnvalue (Components|GetOwner _draggingcomponent))
  (bind _returnvalue_2 (Transformation|GetActorLocation _returnvalue))
  (bind (_x _y _z) (Math|Vector|BreakVector _returnvalue_2))
  (if (Variables|Default|GetIsDragging?)
    (if (not (Variables|/Game/Blueprints/ActorComponents/BPAC_Draggable.BPAC_Draggable_C|GetLockZoom (Variables|Default|GetDraggingComponent)))
      (Utilities|IsValid _draggingcomponent
        (:Is%20Valid
          (bind _camera (Class|BPICamera|GetCamera(Message) (Variables|Default|GetGameState)))
          (Transformation|SetActorLocation _returnvalue (Math|Vector|MakeVector (Math|Float|Clamp(Float) (+ AxisValue _x) (+ (Variables|Default|GetReelMin) (.X (Math|Vector|BreakVector (Transformation|GetActorLocation _camera)))) (+ (.X (Math|Vector|BreakVector (Transformation|GetActorLocation _camera))) (Variables|Default|GetReelMax))) _y _z) false false))))))

(fn ConstructionScript)

(fn GetClickComponent
  (bind (_result _success_) (Utilities|HitDetection))
  (bind _hitactor (Collision|BreakHitResult _result))
  (if _success_
    (Utilities|IsValid _hitactor
      (:Is%20Valid
        (for _array_element (Class|Actor|GetComponentsbyInterface _hitactor "/Script/FGGP2.InteractInterface")
          (Class|InteractInterface|Clickable(Message) _array_element))))))

(fn GetDragComponent
  (bind (_result _success_) (Utilities|HitDetection))
  (bind (_bblockinghit _binitialoverlap _time _distance _location _impactpoint _normal _impactnormal _physmat _hitactor) (Collision|BreakHitResult _result))
  (bind _returnvalue (Actor|GetComponentbyClass _hitactor "/Game/Blueprints/ActorComponents/BPAC_Draggable.BPAC_Draggable_C"))
  (if _success_
    (if (Utilities|IsValid _hitactor)
      (Utilities|IsValid _returnvalue
        (:Is%20Valid
          (bind _output_get (Variables|Default|SetDraggingComponent _returnvalue))
          (Variables|/Game/Blueprints/ActorComponents/BPAC_Draggable.BPAC_Draggable_C|SetDragOffset _returnvalue (- _location (Transformation|GetActorLocation _hitactor)))
          (Class|BPIDraggableInterface|StartDragging(Message) _output_get))))))

(fn GetMemoryObject
  (bind (_result _success_) (Utilities|HitDetection))
  (bind _hitactor (Collision|BreakHitResult _result))
  (bind _returnvalue (Actor|GetComponentbyClass _hitactor "/Game/Blueprints/ActorComponents/BPAC_MemoryObject.BPAC_MemoryObject_C"))
  (if _success_
    (if (Utilities|IsValid _hitactor) ; Did it hit anything?
      (Utilities|IsValid _returnvalue ; Did it hit a BPAC Memory Object?
        (:Is%20Valid
          (bind _asbp_memory_puzzle (Utilities|Casting|CastToBP_MemoryPuzzle (Components|GetOwner _returnvalue)))
          (if (Variables|/Game/Blueprints/Room2/BP_MemoryPuzzle.BP_MemoryPuzzle_C|GetAcceptClicking _asbp_memory_puzzle)
            (bind _output_get (Variables|Default|SetClickedObject _returnvalue))
            (if (not (Variables|/Game/Blueprints/ActorComponents/BPAC_MemoryObject.BPAC_MemoryObject_C|GetCompleted _output_get)) ; Is this memory piece (NOT)\npart of a completed set?
              (Utilities|IsValid (Variables|Default|GetMemoryPuzzleObject) ; Do we have an object stored?
                (:Is%20Valid
                  (if (not (== (Variables|Default|GetMemoryPuzzleObject) (Variables|Default|GetClickedObject))) ; Did we click something OTHER\nthan what we have stored?
                    (Variables|Default|SetAcceptMemoryObjectInput false)
                    (bind _asbp_memory_puzzle_2 (Utilities|Casting|CastToBP_MemoryPuzzle (Components|GetOwner (Variables|Default|GetClickedObject))))
                    (Default|RevealObject _asbp_memory_puzzle_2)
                    (if (== (Variables|/Game/Blueprints/ActorComponents/BPAC_MemoryObject.BPAC_MemoryObject_C|GetMemPuzState (Variables|Default|GetClickedObject)) (Variables|/Game/Blueprints/ActorComponents/BPAC_MemoryObject.BPAC_MemoryObject_C|GetMemPuzState (Variables|Default|GetMemoryPuzzleObject))) ; Do the two objects match?
                      (bind _asbp_memory_puzzle_3 (Utilities|Casting|CastToBP_MemoryPuzzle (Components|GetOwner (Variables|Default|GetClickedObject))))
                      (Default|StayRevealed _asbp_memory_puzzle_3)
                      (bind _asbp_memory_puzzle_4 (Utilities|Casting|CastToBP_MemoryPuzzle (Components|GetOwner (Variables|Default|GetMemoryPuzzleObject))))
                      (Default|StayRevealed _asbp_memory_puzzle_4)
                      (Variables|Default|SetMemoryPuzzleObject 0)
                      (Variables|Default|SetMemoryPuzzlesCompleted (+ 1 (Variables|Default|GetMemoryPuzzlesCompleted)))
                      (Variables|Default|SetCompletedAMemoryPuzzle true)
                      (return false) ; All things matched!
                      (else
                        (return true) ; Failed to match, reset objects
                      ))))
                (:Is%20Not%20Valid
                  (bind _asbp_memory_puzzle_5 (Utilities|Casting|CastToBP_MemoryPuzzle (Components|GetOwner (Variables|Default|GetClickedObject))))
                  (Default|RevealObject _asbp_memory_puzzle_5)
                  (Variables|Default|SetMemoryPuzzleObject (Variables|Default|GetClickedObject))
                  (return false) ; Added 1st stored object
                )))))))))

(fn HideMemoryObjects
  (params (HideObjects :type Boolean))
  (if HideObjects
    (bind _asbp_memory_puzzle (Utilities|Casting|CastToBP_MemoryPuzzle (Components|GetOwner (Variables|Default|GetMemoryPuzzleObject))))
    (Default|HideObject _asbp_memory_puzzle)
    (bind _asbp_memory_puzzle_2 (Utilities|Casting|CastToBP_MemoryPuzzle (Components|GetOwner (Variables|Default|GetClickedObject))))
    (Default|HideObject _asbp_memory_puzzle_2)
    (Variables|Default|SetMemoryPuzzleObject 0)))

(fn CursorLogic
  (bind (_result _success_) (Utilities|HitDetection))
  (bind _gamemode (Variables|Default|GetGameMode))
  (bind _gamemode_2 (Variables|Default|GetGameMode))
  (bind _draggingcomponent (Variables|Default|GetDraggingComponent))
  (bind _hitactor (Collision|BreakHitResult _result))
  (bind _cursorwidget (Variables|/Game/Blueprints/Core/GM_PointAndClick.GM_PointAndClick_C|GetCursorWidget _gamemode))
  (bind _cursorwidget_2 (Variables|/Game/Blueprints/Core/GM_PointAndClick.GM_PointAndClick_C|GetCursorWidget _gamemode_2))
  (if (Utilities|IsValid _cursorwidget_2)
    (if (not (Utilities|IsValid _draggingcomponent))
      (if _success_
        (if (Utilities|IsValid _hitactor)
          ;[1 1 1] Checking every component the hit actor has
          (bind _array_element (Utilities|Array|ForEachLoopwithBreak (Actor|GetComponentsByClass _hitactor "/Script/Engine.ActorComponent") :!label _label)
            (:LoopBody
              ;[1 1 1] Checking every component that we want cursor to react to
              (bind _array_element_2 (Utilities|Array|ForEachLoopwithBreak (Variables|Default|GetActorComponents) :!label _label_2)
                (:LoopBody
                  (if (== _array_element_2 (Utilities|GetClass _array_element))
                    (LocalVariables|SetFoundMatchingComponent true)
                    (goto _label_2 Break)))
                (:Completed
                  (if (LocalVariables|GetFoundMatchingComponent)
                    (goto _label Break)))))
            (:Completed
              (if (LocalVariables|GetFoundMatchingComponent)
                (Default|ClickableCursor _cursorwidget true)
                (else
                  (Default|ClickableCursor _cursorwidget false :!label _label_3)))))
          (else
            (goto _label_3))))
      (elif (Variables|/Script/FGGP2.InteractBaseComponent|Getinteractable _draggingcomponent)
        (Default|DraggingCursor _cursorwidget_2)))))

(fn HoverableEmissive
  (bind (_result _success_) (Utilities|HitDetection))
  (bind _hitactor (Collision|BreakHitResult _result))
  (if _success_
    (if (Utilities|IsValid _hitactor)
      (if (Utilities|DoesObjectImplementInterface _hitactor "/Game/Blueprints/Interfaces/BPI_HoverableEmission.BPI_HoverableEmission_C")
        (if (!= (Variables|Default|GetCurrentlyHoveredEmissive) _hitactor)
          (if (Utilities|IsValid (Variables|Default|GetCurrentlyHoveredEmissive))
            (Class|BPIHoverableEmission|StopHovering(Message) (Variables|Default|GetCurrentlyHoveredEmissive))
            (else
              (Variables|Default|SetCurrentlyHoveredEmissive 0)))
          (Variables|Default|SetCurrentlyHoveredEmissive _hitactor)
          (Class|BPIHoverableEmission|StartHovering(Message) (Variables|Default|GetCurrentlyHoveredEmissive))
          (else
            (Variables|Default|SetCurrentlyHoveredEmissive _hitactor)
            (Class|BPIHoverableEmission|StartHovering(Message) (Variables|Default|GetCurrentlyHoveredEmissive))))
        (else
          (if (Utilities|IsValid (Variables|Default|GetCurrentlyHoveredEmissive)) :!label _label
            (Class|BPIHoverableEmission|StopHovering(Message) (Variables|Default|GetCurrentlyHoveredEmissive))
            (Variables|Default|SetCurrentlyHoveredEmissive 0))))
      (else
        (goto _label)))
    (else
      (goto _label))))