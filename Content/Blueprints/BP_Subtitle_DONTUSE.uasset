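; BP_Subtitle_DONTUSE is a subtitle Blueprint, marked as not for use, that shows timed dialogue lines through a Subtitles widget.
; Start, next and stop functions drive the widget, with only next-line playing sound, at world origin.
; ManageText starts a timer for fixed-duration trigger types, including duration-or-click.
; Event handlers, including Clickable, are empty stubs, and a macro provides a manually advanced index loop.
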(event Custom|SubtitleEventSwitch
  (params (SubtitleEvent :type ESubtitleEvent%20Enum :default "SubtitleFinished")))

(event EventClickable)

(event EventBeginPlay)

(fn StartShowingText
  (Class|BPITextBoxInterface|ShowWidget(Message) (Variables|Default|GetSubtitles))
  (bind _returnvalue (Class|SubtitleComponent|GetCurrentTextData))
  (Class|BPITextBoxInterface|SetText(Message) (Variables|Default|GetSubtitles) (.line (Utilities|Struct|BreakTextData _returnvalue)))
  (CallFunction|ManageText))

(fn StopShowingText
  (bind _subtitles (Variables|Default|GetSubtitles))
  (Class|BPITextBoxInterface|HideWidget(Message) _subtitles)
  (Class|BPITextBoxInterface|ClearText(Message) _subtitles))

(fn NewTexttoShow
  (bind _returnvalue (Class|SubtitleComponent|GetCurrentTextData))
  (Class|BPITextBoxInterface|SetText(Message) (Variables|Default|GetSubtitles) (.line (Utilities|Struct|BreakTextData _returnvalue)))
  (Audio|PlaySoundatLocation (.soundRef (Utilities|Struct|BreakTextData _returnvalue)) "0, 0, 0" "0, 0, 0" 1.0 1.0 0.0 0 0 0)
  (CallFunction|ManageText))

(fn ManageText
  (bind _returnvalue (Class|SubtitleComponent|GetCurrentTextData))
  (switch Utilities|FlowControl|Switch|SwitchonENextLineTrigger (.triggerType (Utilities|Struct|BreakTextData _returnvalue))
    (:OnFixedDuration
      _)
    (:OnFixedDurationOrClick
      _))
  (Class|SubtitleComponent|StartTimer (.duration (Utilities|Struct|BreakTextData _returnvalue))))